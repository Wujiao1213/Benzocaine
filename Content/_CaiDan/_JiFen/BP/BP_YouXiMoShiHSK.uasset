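; BP_YouXiMoShiHSK is a helper that persists the game mode (MoShi) in a HuaMianSheZhi_CunDan save object.
; GetMoShi loads the slot and returns the stored mode, creating and saving a default object when none exists.
; SetMoShi writes a new mode to the loaded or newly created object, saves it to the same slot and returns the save result.
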(fn `GetMoShi`
  (returns (MoShi :type Integer))
  (locals (SlotName :type String :default "HuaMianSheZhi"))
  (bind _returnvalue (`GameplayStatics.DoesSaveGameExist` (`local.SlotName`)))
  (if _returnvalue
    (bind _returnvalue_2 (`GameplayStatics.LoadGameFromSlot` (`local.SlotName`)))
    (bind _ashua_mian_she_zhi_cun_dan (cast `/Game/_CaiDan/CunDan/HuaMianSheZhi_CunDan` _returnvalue_2))
    (return (`/Game/_CaiDan/CunDan/HuaMianSheZhi_CunDan.MoShi` _ashua_mian_she_zhi_cun_dan))
    (else
      (bind _returnvalue_3 (`GameplayStatics.CreateSaveGameObject` "/Game/_CaiDan/CunDan/HuaMianSheZhi_CunDan.HuaMianSheZhi_CunDan_C"))
      (`GameplayStatics.SaveGameToSlot` _returnvalue_3 (`local.SlotName`))
      (return (`/Game/_CaiDan/CunDan/HuaMianSheZhi_CunDan.MoShi` _returnvalue_3)))))

(fn `SetMoShi`
  (params (XinMoShi :type Integer))
  (returns (ChengGong :type Boolean))
  (locals (SlotName :type String :default "HuaMianSheZhi"))
  (bind _returnvalue (`GameplayStatics.DoesSaveGameExist` (`local.SlotName`)))
  (if _returnvalue
    (bind _returnvalue_2 (`GameplayStatics.LoadGameFromSlot` (`local.SlotName`)))
    (bind _ashua_mian_she_zhi_cun_dan (cast `/Game/_CaiDan/CunDan/HuaMianSheZhi_CunDan` _returnvalue_2))
    (set `/Game/_CaiDan/CunDan/HuaMianSheZhi_CunDan.MoShi` (`local.XinMoShi`) _ashua_mian_she_zhi_cun_dan)
    (bind _returnvalue_3 (`GameplayStatics.SaveGameToSlot` _ashua_mian_she_zhi_cun_dan (`local.SlotName`)))
    (return _returnvalue_3)
    (else
      (bind _returnvalue_4 (`GameplayStatics.CreateSaveGameObject` "/Game/_CaiDan/CunDan/HuaMianSheZhi_CunDan.HuaMianSheZhi_CunDan_C"))
      (set `/Game/_CaiDan/CunDan/HuaMianSheZhi_CunDan.MoShi` (`local.XinMoShi`) _returnvalue_4)
      (bind _returnvalue_5 (`GameplayStatics.SaveGameToSlot` _returnvalue_4 (`local.SlotName`)))
      (return _returnvalue_5))))