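; Score component (JiFenZuJian) that tracks the current score, handles point deductions and warns the player.
; On BeginPlay it reads the mode from the display-settings save, which decides whether the score widget is shown.
; JianFen subtracts points with a sound and camera shake, then updates that widget.
; Separately, JianFenUI pops a warning widget and, for all but one tip type, logs the reason, points and step.
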(event `self.ReceiveBeginPlay`
  (`self.YouXiMoShiCSH`))

(fn `JianFen`
  (params (Fen :type Integer))
  (returns (DanQianFenShu :type Integer))
  (if (== Fen 100)
    (`GameplayStatics.PlaySound2D` "/Game/Sounds/error.error" 1.0 1.0 0.0 null null)
    (else
      (`GameplayStatics.PlaySound2D` "/Game/Sounds/warming.warming" 1.0 1.0 0.0 null null)))
  (`PlayerCameraManager.StartCameraShake` :`self` (`PlayerController.PlayerCameraManager` (`GameplayStatics.GetPlayerController` 0)) :`ShakeClass` "/Game/BluePrints/Gamemode/BP_CameraShake.BP_CameraShake_C")
  (set `self.DanQianFenShu` (- (`self.DanQianFenShu`) Fen))
  (bind _w_jifen (`self.W_JiFen`)
    (:`then`
      (`/Game/_CaiDan/_JiFen/UI/W_JiFenJieMian.JianFen` _w_jifen (`KismetTextLibrary.Conv_IntToText` (`local.Fen`)) self)
      (return (`self.DanQianFenShu`)))
    (:`else`)))

(fn `JianFenUI`
  (params (tipsType :type Integer) (tipsText :type Text) (score :type Integer) (step :type Integer))
  (if (not (== tipsType 1))
    (`KismetArrayLibrary.Array_Add` (`self.JianFenXiangShuZu`) (make `/Game/_CaiDan/_JiFen/Struct/F_JianFenXiangQin` tipsText score step))
    (if true
      _
      (else
        _)))
  (bind _returnvalue (`|CreateWidget` "/Game/UI/WBP_Warming.WBP_Warming_C" null tipsType tipsText score))
  (`UserWidget.AddToViewport` _returnvalue 0))

(fn `YouXiMoShiCSH`
  (locals (SlotName :type String :default "HuaMianSheZhi"))
  (bind _w_jifen (`self.W_JiFen`))
  (bind _returnvalue (`GameplayStatics.DoesSaveGameExist` (`local.SlotName`)))
  (if _returnvalue
    (bind _returnvalue_2 (`GameplayStatics.LoadGameFromSlot` (`local.SlotName`)))
    (bind _ashua_mian_she_zhi_cun_dan (cast `/Game/_CaiDan/CunDan/HuaMianSheZhi_CunDan` _returnvalue_2))
    (switch `int` (`/Game/_CaiDan/CunDan/HuaMianSheZhi_CunDan.MoShi` _ashua_mian_she_zhi_cun_dan)
      (:`0`
        (`/Engine/EditorBlueprintResources/StandardMacros.IsValid` _w_jifen
          (:`Is Valid`
            (`Widget.RemoveFromParent` _w_jifen))))
      (:`1`
        (`/Engine/EditorBlueprintResources/StandardMacros.IsValid` _w_jifen
          (:`Is Valid`
            _)
          (:`Is Not Valid`
            (bind _returnvalue_3 (`|CreateWidget` "/Game/_CaiDan/_JiFen/UI/W_JiFenJieMian.W_JiFenJieMian_C"))
            (bind _output_get (set `self.W_JiFen` _returnvalue_3))))
        (`/Game/_CaiDan/_JiFen/UI/W_JiFenJieMian.SetFenShu` _output_get (`KismetTextLibrary.Conv_IntToText` (`self.DanQianFenShu`)))
        (`UserWidget.AddToViewport` (`self.W_JiFen`) 0)))
    (else
      (bind _returnvalue_4 (`GameplayStatics.CreateSaveGameObject` "/Game/_CaiDan/CunDan/HuaMianSheZhi_CunDan.HuaMianSheZhi_CunDan_C"))
      (switch `int` (`/Game/_CaiDan/CunDan/HuaMianSheZhi_CunDan.MoShi` _returnvalue_4)
        (:`1`
          (bind _returnvalue_5 (`|CreateWidget` "/Game/_CaiDan/_JiFen/UI/W_JiFenJieMian.W_JiFenJieMian_C"))
          (bind _output_get_2 (set `self.W_JiFen` _returnvalue_5))
          (`/Game/_CaiDan/_JiFen/UI/W_JiFenJieMian.SetFenShu` _output_get_2 (`KismetTextLibrary.Conv_IntToText` (`self.DanQianFenShu`)))
          (`UserWidget.AddToViewport` (`self.W_JiFen`) 0)
          (`GameplayStatics.SaveGameToSlot` _returnvalue_4 (`local.SlotName`)))))))