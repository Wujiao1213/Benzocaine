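; Blueprint for a 5 ml graduated cylinder (LiangTong) that can be inspected up close in a separate studio actor.
; CheakActor spawns a BP_Studio at a far-off location, out of the level's way, and passes it the OutLineMesh static mesh to focus on.
; The Destroy event removes that studio instance and clears the reference.
; BeginPlay, overlap, Tick and the construction script add no logic.
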(event `CheakActor`
  (bind _returnvalue (`|SpawnActorFromClass` "/Game/BulePrints/BP_Studio.BP_Studio_C" (`KismetMathLibrary.MakeTransform` (100000000.0 0.0 0.0)) "Undefined" "MultiplyWithRoot" null null))
  (bind _output_get (set `self.BP_Studio_0` _returnvalue))
  (`/Game/BulePrints/BPI_Inspect.Inspect` _output_get null (`StaticMeshComponent.StaticMesh` (`self.OutLineMesh`))))

(event `/Game/BulePrints/BPI_Inspect.Destroy`
  (bind _bp_studio_0 (`self.BP_Studio_0`))
  (`/Engine/EditorBlueprintResources/StandardMacros.IsValid` _bp_studio_0
    (:`Is Valid`
      (`/Game/BulePrints/BPI_Inspect.Destroy` _bp_studio_0)
      (set `self.BP_Studio_0` null))))

(fn `UserConstructionScript`
  (`parent.UserConstructionScript`))