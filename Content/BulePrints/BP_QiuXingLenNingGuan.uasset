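; BP_QiuXingLenNingGuan is a spherical condenser tube actor (pinyin name) with two cable components, Cable and Cable1.
; On BeginPlay it attaches the end of each cable to the child actor of its matching component, CableEnd or CableEnd1.
; The overlap and tick events are disabled, and the construction script only calls its parent.
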(event `self.ReceiveBeginPlay`
  (`parent.ReceiveBeginPlay`)
  (`CableComponent.SetAttachEndTo` (`self.Cable`) (`ChildActorComponent.ChildActor` (`self.CableEnd`)) "None" "None")
  (`CableComponent.SetAttachEndTo` (`self.Cable1`) (`ChildActorComponent.ChildActor` (`self.CableEnd1`)) "None" "None"))

(fn `UserConstructionScript`
  (`parent.UserConstructionScript`))