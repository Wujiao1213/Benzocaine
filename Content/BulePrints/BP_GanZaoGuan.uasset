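; Drying tube (GanZaoGuan) lab prop that can be equipped and packed with cotton and a ClCa sphere, apparently calcium chloride.
; Events reveal the fillings and set step flags, and show, hide or refresh its widget panel.
; While equipped, overlap tracks the other actor, and targeting dispatches on its class name to add cotton.
; Equip, quit and cotton insertion play Level Sequence frame ranges, with Step2 choosing the cotton animation.
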(event `self.ReceiveBeginPlay`
  (`parent.ReceiveBeginPlay`))

(event `VisApplication`
  (`SceneComponent.SetVisibility` (`self.Application`) true false))

(event `DisApplication`
  (`SceneComponent.SetVisibility` (`self.Application`) false false))

(event `VisClCa`
  (if (not (`self.Step3`))
    (`SceneComponent.SetVisibility` (`self.Sphere`) true false)
    (set `self.Step2` true)))

(event `VisMH1`
  (`SceneComponent.SetVisibility` (`self.Mianhua1`) true false)
  (set `self.Step1` true))

(event `VisMH2`
  (`SceneComponent.SetVisibility` (`self.Mianhua2`) true false))

(event `UpdateView`
  (bind _aswbp_gan_zao_guan_app (cast `/Game/UI/Actor/WBP_GanZaoGuan_APP` (`WidgetComponent.GetUserWidgetObject` (`self.Application`))))
  (`/Game/UI/Actor/WBP_GanZaoGuan_APP.UpdateView` _aswbp_gan_zao_guan_app))

(event `AddMianhua`
  (bind _sequenceplayer (`LevelSequenceActor.SequencePlayer` (`self.LS_MianHua`)))
  (bind _sequenceplayer_2 (`LevelSequenceActor.SequencePlayer` (`self.LS_A`)))
  (if (`self.Step2`)
    (`MovieSceneSequencePlayer.SetPlaybackPosition` _sequenceplayer_2 (make `MovieSceneSequencePlaybackParams` (make `FrameTime` (make `FrameNumber` 320)) 0.0 "" "Frame" "Jump"))
    (`MovieSceneSequencePlayer.SetPlaybackPosition` (`LevelSequenceActor.SequencePlayer` (`self.LS_MianHua1`)) (make `MovieSceneSequencePlaybackParams` (make `FrameTime` (make `FrameNumber` 320)) 0.0 "" "Frame" "Jump"))
    (`MovieSceneSequencePlayer.PlayTo` :`self` _sequenceplayer_2 :`PlaybackParams` (make `MovieSceneSequencePlaybackParams` (make `FrameTime` (make `FrameNumber` 370))))
    (`MovieSceneSequencePlayer.PlayTo` :`self` (`LevelSequenceActor.SequencePlayer` (`self.LS_MianHua1`)) :`PlaybackParams` (make `MovieSceneSequencePlaybackParams` (make `FrameTime` (make `FrameNumber` 370))))
    (else
      (`MovieSceneSequencePlayer.SetPlaybackPosition` _sequenceplayer (make `MovieSceneSequencePlaybackParams` (make `FrameTime` (make `FrameNumber` 30)) 0.0 "" "Frame" "Jump"))
      (`MovieSceneSequencePlayer.SetPlaybackPosition` _sequenceplayer_2 (make `MovieSceneSequencePlaybackParams` (make `FrameTime` (make `FrameNumber` 30)) 0.0 "" "Frame" "Jump"))
      (`MovieSceneSequencePlayer.PlayTo` :`self` _sequenceplayer :`PlaybackParams` (make `MovieSceneSequencePlaybackParams` (make `FrameTime` (make `FrameNumber` 90))))
      (`MovieSceneSequencePlayer.PlayTo` :`self` _sequenceplayer_2 :`PlaybackParams` (make `MovieSceneSequencePlaybackParams` (make `FrameTime` (make `FrameNumber` 90)))))))

(event `Equie`
  (bind _sequenceplayer (`LevelSequenceActor.SequencePlayer` (`self.LS_A`)))
  (`MovieSceneSequencePlayer.SetPlaybackPosition` _sequenceplayer (make `MovieSceneSequencePlaybackParams` (make `FrameTime` (make `FrameNumber` 0))))
  (`MovieSceneSequencePlayer.PlayTo` :`self` _sequenceplayer :`PlaybackParams` (make `MovieSceneSequencePlaybackParams` (make `FrameTime` (make `FrameNumber` 30)))))

(event `Quit`
  (bind _sequenceplayer (`LevelSequenceActor.SequencePlayer` (`self.LS_A`)))
  (if (< (break `FrameNumber` (break `QualifiedFrameTime` (`MovieSceneSequencePlayer.GetCurrentTime` _sequenceplayer))) 29)
    (`MovieSceneSequencePlayer.SetPlaybackPosition` _sequenceplayer (make `MovieSceneSequencePlaybackParams` (make `FrameTime` (make `FrameNumber` 1)) 0.0 "" "Frame" "Jump"))
    (else
      (`MovieSceneSequencePlayer.SetPlaybackPosition` _sequenceplayer (make `MovieSceneSequencePlaybackParams` (make `FrameTime` (make `FrameNumber` 30)) 0.0 "" "Frame" "Jump"))))
  (`MovieSceneSequencePlayer.PlayTo` :`self` _sequenceplayer :`PlaybackParams` (make `MovieSceneSequencePlaybackParams` (make `FrameTime` (make `FrameNumber` 0)))))

(event `self.FindOtherBP_Thing.OnComponentBeginOverlap`
  (params (OverlappedComponent :type "PrimitiveComponent Object Reference") (OtherActor :type "Actor Object Reference") (OtherComp :type "PrimitiveComponent Object Reference") (OtherBodyIndex :type Integer) (bFromSweep :type Boolean) (SweepResult :type "HitResult Structure (by ref)"))
  (if (`self.IsEquitState`)
    (set `self.Other Actor` OtherActor)
    (set `self.HasPositionUpdate` true)))

(event `self.FindOtherBP_Thing.OnComponentEndOverlap`
  (params (OverlappedComponent :type "PrimitiveComponent Object Reference") (OtherActor :type "Actor Object Reference") (OtherComp :type "PrimitiveComponent Object Reference") (OtherBodyIndex :type Integer))
  (if (`self.IsEquitState`)
    (set `self.Other Actor` null)
    (set `self.HasPositionUpdate` false)))

(event `self.ThingTargeEvent`
  (bind _returnvalue (`KismetSystemLibrary.GetClassDisplayName` (`GameplayStatics.GetObjectClass` (`self.Other Actor`))))
  (switch `name` (`KismetStringLibrary.Conv_StringToName` _returnvalue)
    (:`Default`
      (`KismetSystemLibrary.PrintString` _returnvalue))
    (:`BP_MianHua_C`
      (`self.AddMianhua`))))

(fn `Init`)

(fn `OffOutLine`
  (`parent.OffOutLine`))

(fn `OnOutLine`
  (`parent.OnOutLine`))

(fn `UserConstructionScript`
  (`parent.UserConstructionScript`))