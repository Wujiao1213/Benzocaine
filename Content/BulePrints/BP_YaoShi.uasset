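; BP_YaoShi is a medicine spoon (药匙) actor with a toggleable powder (Fenmo) component.
; The VisFenMo event shows or hides that powder.
; When the FindOtherBP_Thing component begins overlapping a BP_ClCa, the Details widget's label changes to "取用" (take).
; Any end overlap on that component resets the label to "药匙", without checking the other actor's class.
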(event `VisFenMo`
  (params (vis :type Boolean))
  (`SceneComponent.SetVisibility` (`self.fenmo`) vis false))

(event `self.FindOtherBP_Thing.OnComponentBeginOverlap`
  (params (OverlappedComponent :type "PrimitiveComponent Object Reference") (OtherActor :type "Actor Object Reference") (OtherComp :type "PrimitiveComponent Object Reference") (OtherBodyIndex :type Integer) (bFromSweep :type Boolean) (SweepResult :type "HitResult Structure (by ref)"))
  (if (== (`GameplayStatics.GetObjectClass` OtherActor) "/Game/BulePrints/BP_ClCa.BP_ClCa_C")
    (bind _aswbp_details (cast `/Game/UI/WBP_Details` (`WidgetComponent.GetUserWidgetObject` (`self.Details`))))
    (`/Game/UI/Child/WBP_Name.Set Text` (`/Game/UI/WBP_Details.WBP_Name` _aswbp_details) "取用")))

(event `self.FindOtherBP_Thing.OnComponentEndOverlap`
  (params (OverlappedComponent :type "PrimitiveComponent Object Reference") (OtherActor :type "Actor Object Reference") (OtherComp :type "PrimitiveComponent Object Reference") (OtherBodyIndex :type Integer))
  (bind _aswbp_details (cast `/Game/UI/WBP_Details` (`WidgetComponent.GetUserWidgetObject` (`self.Details`))))
  (`/Game/UI/Child/WBP_Name.Set Text` (`/Game/UI/WBP_Details.WBP_Name` _aswbp_details) "药匙"))

(fn `UserConstructionScript`
  (`parent.UserConstructionScript`))