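; Reagent cabinet (ShiJiGui) actor whose right handle component swings open and closed.
; Open and Close events play and reverse one timeline, which drives the handle's relative yaw across a 90-degree scale.
; The timeline sets an Opening flag while moving in either direction, then clears it and toggles OpenOrClose when finished.
; BeginPlay, Tick, overlap and construction add no logic of their own.
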(event `Open`
  (bind (_direction _rotation) (`Timeline|时间轴_0` :!label _label)
    (:`Update`
      (set `self.Opening` true)
      (`SceneComponent.K2_SetRelativeRotation` (`self.SM_ShiJiGui_HandleRight`) (`KismetMathLibrary.MakeRotator` 0.0 0.0 (* _rotation 90.0)) false false))
    (:`Finished`
      (set `self.OpenOrClose` (not (`self.OpenOrClose`)))
      (set `self.Opening` false))))

(event `Close`
  (goto _label :!via `Reverse`))

(fn `UserConstructionScript`
  (`parent.UserConstructionScript`))