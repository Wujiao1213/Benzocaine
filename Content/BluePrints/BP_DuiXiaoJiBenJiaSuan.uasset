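; Actor Blueprint for a lab item, apparently p-nitrobenzoic acid going by its pinyin name, that reacts to contact with BP_Cheng.
; An overlap on its FindOtherBP_Thing component checks for that exact class, then resets the LSDuijiXiao sequence player's playback position and plays it to a fixed frame.
; BeginPlay, ActorBeginOverlap and the construction script add no logic of their own.
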(event `self.FindOtherBP_Thing.OnComponentBeginOverlap`
  (params (OverlappedComponent :type "PrimitiveComponent Object Reference") (OtherActor :type "Actor Object Reference") (OtherComp :type "PrimitiveComponent Object Reference") (OtherBodyIndex :type Integer) (bFromSweep :type Boolean) (SweepResult :type "HitResult Structure (by ref)"))
  (bind _sequenceplayer (`LevelSequenceActor.SequencePlayer` (`self.LS_DuijiXiao`)))
  (if (== (`GameplayStatics.GetObjectClass` OtherActor) "/Game/BluePrints/BP_Cheng.BP_Cheng_C")
    (`MovieSceneSequencePlayer.SetPlaybackPosition` _sequenceplayer (make `MovieSceneSequencePlaybackParams` (make `FrameTime` (make `FrameNumber` 0))))
    (`MovieSceneSequencePlayer.PlayTo` :`self` _sequenceplayer :`PlaybackParams` (make `MovieSceneSequencePlaybackParams` (make `FrameTime` (make `FrameNumber` 40))))))

(fn `UserConstructionScript`
  (`parent.UserConstructionScript`))