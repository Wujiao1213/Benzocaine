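; BP_Studio2 is an inspection studio actor that displays a copy of a BP_Thing alongside selectable graduated cylinders (量筒).
; Inspect spawns that class through a child actor component, copies its Name, opens WBP_Inspect2 linked back to the studio, and sets the player controller's InUnableMoveUi flag.
; ChangeLT shows one cylinder and water mesh pair by capacity index, hiding the others and storing the pair in UseMesh and UseWater.
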(event `self.ReceiveBeginPlay`
  (set `self.useMesh` (`self.5ml量筒`))
  (set `self.useWater` (`self.5w`)))

(event `/Game/BluePrints/Gamemode/BPI_Inspect.Inspect`
  (params (Player :type "/Game/Characters/FirstPerson/Blueprints/BP_FirstPersonCharacter Object Reference") (WhichItemToFocus :type "StaticMesh Object Reference") (ChildActor :type "Actor Object Reference"))
  (bind _childactor (`self.ChildActor`))
  (set `self.TrgetActor` ChildActor)
  (`ChildActorComponent.SetChildActorClass` _childactor (`GameplayStatics.GetObjectClass` ChildActor))
  (bind _asbp_thing (cast `/Game/BluePrints/BP_Thing` ChildActor))
  (bind _asbp_thing_2 (cast `/Game/BluePrints/BP_Thing` (`ChildActorComponent.ChildActor` _childactor)))
  (set `/Game/BluePrints/BP_Thing.Name` (`/Game/BluePrints/BP_Thing.Name` _asbp_thing) _asbp_thing_2)
  (bind _returnvalue (`|CreateWidget` "/Game/UI/WBP_Inspect2.WBP_Inspect2_C"))
  (set `/Game/UI/WBP_Inspect2.ParentActor` self _returnvalue)
  (bind _output_get (set `self.WBP_Inspect2` _returnvalue))
  (set `self.ParentActor` self)
  (`UserWidget.AddToViewport` _output_get 0)
  (bind _asbp_first_person_player_control (cast `/Game/Characters/FirstPerson/Blueprints/BP_FirstPersonPlayerControl` (`GameplayStatics.GetPlayerController` 0)))
  (set `/Game/Characters/FirstPerson/Blueprints/BP_FirstPersonPlayerControl.InUnableMoveUi` true _asbp_first_person_player_control))

(event `/Game/BluePrints/Gamemode/BPI_Inspect.Destroy`
  (`self.K2_DestroyActor`))

(event `ChangeLT`
  (params (`容量` :type Integer))
  (bind `_5ml量筒` (`self.5ml量筒`))
  (bind `_10ml量筒` (`self.10ml量筒`))
  (bind `_50ml量筒` (`self.50ml量筒`))
  (bind `_25ml量筒` (`self.25ml量筒`))
  (switch `int` `容量`
    (:`0`
      (`SceneComponent.SetVisibility` `_5ml量筒` true false)
      (`SceneComponent.SetVisibility` (`self.5w`) true false)
      (`SceneComponent.SetVisibility` `_10ml量筒` false false)
      (`SceneComponent.SetVisibility` `_50ml量筒` false false)
      (`SceneComponent.SetVisibility` `_25ml量筒` false false)
      (`SceneComponent.SetVisibility` (`self.10w`) false false)
      (`SceneComponent.SetVisibility` (`self.25w`) false false)
      (`SceneComponent.SetVisibility` (`self.50w`) false false)
      (set `self.useMesh` `_5ml量筒`)
      (set `self.useWater` (`self.5w`)))
    (:`1`
      (`SceneComponent.SetVisibility` `_10ml量筒` true false)
      (`SceneComponent.SetVisibility` (`self.10w`) true false)
      (`SceneComponent.SetVisibility` `_5ml量筒` false false)
      (`SceneComponent.SetVisibility` `_50ml量筒` false false)
      (`SceneComponent.SetVisibility` `_25ml量筒` false false)
      (`SceneComponent.SetVisibility` (`self.5w`) false false)
      (`SceneComponent.SetVisibility` (`self.25w`) false false)
      (`SceneComponent.SetVisibility` (`self.50w`) false false)
      (set `self.useMesh` `_10ml量筒`)
      (set `self.useWater` (`self.10w`)))
    (:`2`
      (`SceneComponent.SetVisibility` `_25ml量筒` true false)
      (`SceneComponent.SetVisibility` (`self.25w`) true false)
      (`SceneComponent.SetVisibility` `_5ml量筒` false false)
      (`SceneComponent.SetVisibility` `_10ml量筒` false false)
      (`SceneComponent.SetVisibility` `_50ml量筒` false false)
      (`SceneComponent.SetVisibility` (`self.5w`) false false)
      (`SceneComponent.SetVisibility` (`self.10w`) false false)
      (`SceneComponent.SetVisibility` (`self.50w`) false false)
      (set `self.useMesh` `_25ml量筒`)
      (set `self.useWater` (`self.25w`)))
    (:`3`
      (`SceneComponent.SetVisibility` `_50ml量筒` true false)
      (`SceneComponent.SetVisibility` (`self.50w`) true false)
      (`SceneComponent.SetVisibility` `_5ml量筒` false false)
      (`SceneComponent.SetVisibility` `_10ml量筒` false false)
      (`SceneComponent.SetVisibility` `_25ml量筒` false false)
      (`SceneComponent.SetVisibility` (`self.5w`) false false)
      (`SceneComponent.SetVisibility` (`self.10w`) false false)
      (`SceneComponent.SetVisibility` (`self.25w`) false false)
      (set `self.useMesh` `_50ml量筒`)
      (set `self.useWater` (`self.50w`)))))

(fn `UserConstructionScript`)