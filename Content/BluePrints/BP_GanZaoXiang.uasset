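; Drying oven (GanZaoXiang) actor with an animated door that stores items in slots and converts them to their dried versions.
; A timeline rotates the door, toggles the open state and refreshes the widget's buttons on finish.
; FangRu places items at the first free of six positions, and NaChu clears a slot.
; GanZao0 renames items not flagged as dried using DT_GanZaoWu lookups and updates their detail widgets.
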(event `self.ReceiveBeginPlay`
  (`parent.ReceiveBeginPlay`)
  (`|ExecutionSequence`
    (:`then_0`
      (`KismetArrayLibrary.Array_Add` (`self.WeiZhi`) (`self.1`))
      (`KismetArrayLibrary.Array_Add` (`self.WeiZhi`) (`self.2`))
      (`KismetArrayLibrary.Array_Add` (`self.WeiZhi`) (`self.3`))
      (`KismetArrayLibrary.Array_Add` (`self.WeiZhi`) (`self.4`))
      (`KismetArrayLibrary.Array_Add` (`self.WeiZhi`) (`self.5`))
      (`KismetArrayLibrary.Array_Add` (`self.WeiZhi`) (`self.6`)))
    (:`then_1`
      (bind _aswbp_gan_zao_xiang (cast `/Game/UI/Actor/WBP_GanZaoXiang` (`WidgetComponent.GetWidget` (`self.Application`))))
      (set `self. WBP Gan Zao Xiang` _aswbp_gan_zao_xiang))))

(event `Open`
  (bind (_direction _rotation) (`Timeline|时间轴_opendoor` :!label _label)
    (:`Update`
      (set `self.Opening` true)
      (`SceneComponent.K2_SetRelativeRotation` (`self.Merge_CBC91CD8`) (`KismetMathLibrary.MakeRotator` 0.0 0.0 (* _rotation 90.0)) false false))
    (:`Finished`
      (set `self.OpenOrClose` (not (`self.OpenOrClose`)))
      (set `self.Opening` false)
      (`/Game/UI/Actor/WBP_GanZaoXiang.GenXinAnNiu` (`self. WBP Gan Zao Xiang`)))))

(event `Close`
  (goto _label :!via `Reverse`))

(fn `FangRu`
  (params (BPThing :type "/Game/BluePrints/BP_Thing Object Reference"))
  (returns (ChengGong :type Boolean))
  (bind _bpthing (`local.BPThing`))
  (`/Engine/EditorBlueprintResources/StandardMacros.IsValid` BPThing
    (:`Is Valid`
      (`self.SetActorHiddenInGame` BPThing false)
      (bind (_found _index) (`self.FindNoneSlot`))
      (if _found
        (`KismetArrayLibrary.Array_Set` (`self.BPThingSZ`) _index (`local.BPThing`))
        (set `/Game/BluePrints/BP_Thing.GanZaoXiangIndex` _index _bpthing)
        (`self.K2_SetActorLocation` _bpthing (`SceneComponent.K2_GetComponentLocation` (`|GetArrayItem` (`self.WeiZhi`) _index)) false false)
        (return true)
        (else
          (`KismetSystemLibrary.PrintString` "干燥箱已满")
          (return false))))))

(fn `FindGanZaoWu`
  (params (Name :type Text))
  (returns (Found :type Boolean) (GanZaoWu_Name :type Text))
  (bind _outrownames (`DataTableFunctionLibrary.GetDataTableRowNames` "/Game/Characters/_KuCun/BiaoGe/DT_GanZaoWu.DT_GanZaoWu"))
  (for _array_element _outrownames
    (bind _returnvalue (`|GetDataTableRow` "/Game/Characters/_KuCun/BiaoGe/DT_GanZaoWu.DT_GanZaoWu" _array_element)
      (:`then`
        (bind (_name _ganzaowu_name) (break `/Game/Characters/_KuCun/Struct/F_GanZaoWuPin` _returnvalue))
        (if (`KismetTextLibrary.EqualEqual_TextText` _name Name)
          (return true _ganzaowu_name)))))
  (return false ""))

(fn `FindNoneSlot`
  (returns (Found :type Boolean) (Index :type Integer))
  (for (_array_element _array_index) (`self.BPThingSZ`)
    (`/Engine/EditorBlueprintResources/StandardMacros.IsValid` _array_element
      (:`Is Not Valid`
        (return true _array_index))))
  (return false -1))

(fn `GanZao_0`
  (for _array_element (`self.BPThingSZ`)
    (if (`KismetSystemLibrary.IsValid` _array_element)
      (if (not (`/Game/BluePrints/BP_Thing.GanZao` _array_element))
        (bind (_found _ganzaowu_name) (`self.FindGanZaoWu` (`/Game/BluePrints/BP_Thing.Name` _array_element)))
        (if _found
          (set `/Game/BluePrints/BP_Thing.Name` _ganzaowu_name _array_element)
          (`self.SetDetailsToWidget` _array_element))))))

(fn `NaChu`
  (params (Index :type Integer))
  (`KismetArrayLibrary.Array_Set` (`self.BPThingSZ`) Index))

(fn `UserConstructionScript`
  (`parent.UserConstructionScript`))