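; BP_Studio1 is an inspection stage that shows a copy of a BP_Thing and tilts a medicine spoon (YaoShi).
; Inspect sets the child actor to the target's class, copies its Name, opens WBP_Inspect1 and sets a UI movement-lock flag on the first-person controller.
; A timeline drives the spoon's pitch to pour, and Un reverses it.
; Destroy removes the stage.
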(event `/Game/BluePrints/Gamemode/BPI_Inspect.Inspect`
  (params (Player :type "/Game/Characters/FirstPerson/Blueprints/BP_FirstPersonCharacter Object Reference") (WhichItemToFocus :type "StaticMesh Object Reference") (ChildActor :type "Actor Object Reference"))
  (bind _childactor (`self.ChildActor`))
  (set `self.TrgetActor` ChildActor)
  (`ChildActorComponent.SetChildActorClass` _childactor (`GameplayStatics.GetObjectClass` ChildActor))
  (bind _asbp_thing (cast `/Game/BluePrints/BP_Thing` ChildActor))
  (bind _asbp_thing_2 (cast `/Game/BluePrints/BP_Thing` (`ChildActorComponent.ChildActor` _childactor)))
  (set `/Game/BluePrints/BP_Thing.Name` (`/Game/BluePrints/BP_Thing.Name` _asbp_thing) _asbp_thing_2)
  (bind _returnvalue (`|CreateWidget` "/Game/UI/WBP_Inspect1.WBP_Inspect1_C"))
  (bind _output_get (set `self.WBP_Inspect1` _returnvalue))
  (set `/Game/UI/WBP_Inspect1.ParentActor` self _returnvalue)
  (set `self.ParentActor` self)
  (`UserWidget.AddToViewport` _output_get 0)
  (bind _asbp_first_person_player_control (cast `/Game/Characters/FirstPerson/Blueprints/BP_FirstPersonPlayerControl` (`GameplayStatics.GetPlayerController` 0)))
  (set `/Game/Characters/FirstPerson/Blueprints/BP_FirstPersonPlayerControl.InUnableMoveUi` true _asbp_first_person_player_control))

(event `/Game/BluePrints/Gamemode/BPI_Inspect.Destroy`
  (`self.K2_DestroyActor`))

(event `倾倒药匙`
  (bind (_direction _yaw) (`Timeline|时间轴` :!label _label)
    (:`Update`
      (`SceneComponent.K2_SetRelativeRotation` (`self.YaoShi`) (`KismetMathLibrary.MakeRotator` 0.0 _yaw) false false))))

(event `Un`
  (goto _label :!via `Reverse`))

(fn `UserConstructionScript`)