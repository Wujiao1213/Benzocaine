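; BP_LiangTong_10ml is a 10 ml measuring cylinder actor (liangtong) with a Niagara water level and an inspection view.
; CheakActor spawns a BP_Studio far from the world origin, stores it and passes the cylinder to its Inspect function.
; Destroy removes that studio and clears the reference.
; WaterHight sets the liquid height through the Niagara BottleSize vector, keeping width and depth fixed.
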(event `CheakActor`
  (bind _returnvalue (`|SpawnActorFromClass` "/Game/BluePrints/BP_Studio.BP_Studio_C" (`KismetMathLibrary.MakeTransform` (100000000.0 0.0 0.0)) "Undefined" "MultiplyWithRoot" null null))
  (bind _output_get (set `self.BP_Studio` _returnvalue))
  (`/Game/BluePrints/BPI_Inspect.Inspect` _output_get null null self))

(event `/Game/BluePrints/BPI_Inspect.Destroy`
  (bind _bp_studio (`self.BP_Studio`))
  (`/Engine/EditorBlueprintResources/StandardMacros.IsValid` _bp_studio
    (:`Is Valid`
      (`/Game/BluePrints/BPI_Inspect.Destroy` _bp_studio)
      (set `self.BP_Studio` null))))

(fn `UserConstructionScript`
  (`parent.UserConstructionScript`))

(fn `WaterHight`
  (params (Hight :type "Float (double-precision)"))
  (`NiagaraComponent.SetVariableVec3` (`self.Niagara`) "BottleSize" (`KismetMathLibrary.MakeVector` 12.0 12.0 Hight)))