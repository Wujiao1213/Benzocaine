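; Round-bottom flask actor for the refining (JingZhi) stage of what appears to be a chemistry lab experiment.
; Named step events pour in solids, add 50% ethanol and add activated carbon by playing frame ranges of flask or water-bath Level Sequences through PlayLs, which jumps, then plays to an end frame.
; Other events store the flask in the player's inventory component and reveal a button in WBP_YuanDi_3 for the carbon step.
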(event `RuKu`
  (`/Game/Characters/_KuCun/BP/BP_WanJiaKC.RuKu` (`self.GetComponentByClass` (`GameplayStatics.GetPlayerPawn` 0) "/Game/Characters/_KuCun/BP/BP_WanJiaKC.BP_WanJiaKC_C") self))

(event `显示加入活性炭UI`
  (bind _aswbp_yuan_di_3 (cast `/Game/UI/Actor/JingZhi/WBP_YuanDi_3` (`WidgetComponent.GetUserWidgetObject` (`self.Application`))))
  (set `Widget.Visibility` "Visible" (`/Game/UI/Actor/JingZhi/WBP_YuanDi_3.Button2_2` _aswbp_yuan_di_3)))

(event `倒入所得固体`
  (`self.PlayLs` (`self.LS_JingZhi_YuanDiShaoPing`) 0 30))

(event `加入活性炭`
  (`self.PlayLs` (`self.LS_JingZhi_ShuiYuGuo`) 150 261))

(event `倒入50%乙醇`
  (`self.PlayLs` (`self.LS_JingZhi_YuanDiShaoPing`) 30 91))

(fn `PlayLs`
  (params (LS :type "LevelSequenceActor Object Reference") (Start :type Integer) (End :type Integer))
  (bind _sequenceplayer (`LevelSequenceActor.SequencePlayer` LS))
  (`MovieSceneSequencePlayer.SetPlaybackPosition` _sequenceplayer (make `MovieSceneSequencePlaybackParams` (make `FrameTime` (make `FrameNumber` Start)) 0.0 "" (struct) "Frame" "Jump"))
  (`MovieSceneSequencePlayer.PlayTo` :`self` _sequenceplayer :`PlaybackParams` (make `MovieSceneSequencePlaybackParams` (make `FrameTime` (make `FrameNumber` End)))))

(fn `UserConstructionScript`
  (`parent.UserConstructionScript`))