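; Water bath Blueprint (ShuiYuGuo) for what appears to be a lab apparatus, with a clickable knob and a text display.
; Clicking the knob plays or reverses a rotation timeline, whose completion flips IsOff and switches the display's text and visibility.
; Events for adding a round-bottom flask and bulb condenser play consecutive segments of one level sequence via PlayLs.
; Outline functions defer to the parent; temperature-increase logic is left unconnected.
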(event `self.ReceiveBeginPlay`
  (`parent.ReceiveBeginPlay`))

(event `self.立方体_3_2.OnClicked`
  (params (TouchedComponent :type "PrimitiveComponent Object Reference") (ButtonPressed :type "Key Structure"))
  (bind _textrender (`self.TextRender`))
  (bind _textrender_2 (`self.TextRender`))
  (bind _isoff (`self.IsOff`))
  (if _isoff
    (bind (_direction _rotationz) (`Timeline|按钮旋转` :!via `Reverse` :!label _label)
      (:`Update`
        (`SceneComponent.K2_SetRelativeRotation` (`self.立方体_3_2`) (`KismetMathLibrary.MakeRotator` _rotationz) false false))
      (:`Finished`
        (if _isoff
          (set `self.IsOff` false)
          (`TextRenderComponent.K2_SetText` _textrender_2 (`self.Value_1`))
          (`SceneComponent.SetVisibility` _textrender_2 false false)
          (else
            (set `self.IsOff` true)
            (`TextRenderComponent.K2_SetText` _textrender (`self.Value_2`))
            (`SceneComponent.SetVisibility` _textrender true false)))))
    (else
      (goto _label))))

(event `AddYuanDiShaoPing`
  (`self.PlayLs` (`self.LS_JingZhi_ShuiYuGuan`) 0 90))

(event `AddQiuXingLenNingGuan`
  (`self.PlayLs` (`self.LS_JingZhi_ShuiYuGuan`) 90 150))

(fn `OffOutLine`
  (`parent.OffOutLine`))

(fn `OnOutLine`
  (`parent.OnOutLine`))

(fn `UserConstructionScript`)