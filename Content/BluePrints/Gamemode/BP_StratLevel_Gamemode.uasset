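; BP_StratLevel_Gamemode is the game mode for the start level, handling the non-VR player spawn.
; On BeginPlay, when no head-mounted display is enabled, it spawns a BP_FirstPersonCharacter at a found player start, possesses it with player controller 0 and calls its BindController.
; It has no branch for an enabled headset, and a leftover spawn-and-possess chain with no class set is never run.
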(event `self.ReceiveBeginPlay`
  (if (not (`HeadMountedDisplayFunctionLibrary.IsHeadMountedDisplayEnabled`))
    (bind _returnvalue (`|SpawnActorFromClass` "/Game/Characters/FirstPerson/Blueprints/BP_FirstPersonCharacter.BP_FirstPersonCharacter_C" (`KismetMathLibrary.Conv_VectorToTransform` (`self.K2_GetActorLocation` (`self.K2_FindPlayerStart` null))) "Undefined" "MultiplyWithRoot" null null))
    (`Controller.Possess` (`GameplayStatics.GetPlayerController` 0) _returnvalue)
    (`/Game/Characters/FirstPerson/Blueprints/BP_FirstPersonCharacter.BindController` _returnvalue)))

(fn `UserConstructionScript`)