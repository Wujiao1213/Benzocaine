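; BP_YuanDiShaoPing_2 is an interactable round-bottom flask (圆底烧瓶) that reacts to nearby lab equipment.
; Overlapping an iron stand or beaker relabels its details widget (load or pour) and plays the matching Level Sequence, binding itself at runtime for the beaker's.
; Ending overlap restores the flask name.
; CheakActor spawns a far-off BP_Studio to inspect the flask, and the Destroy event removes that studio.
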(event `CheakActor`
  (bind _returnvalue (`|SpawnActorFromClass` "/Game/BluePrints/BP_Studio.BP_Studio_C" (`KismetMathLibrary.MakeTransform` (100000000.0 0.0 0.0)) "Undefined" "MultiplyWithRoot" null null))
  (bind _output_get (set `self.BP_Studio_0` _returnvalue))
  (`/Game/BluePrints/Gamemode/BPI_Inspect.Inspect` _output_get null null self))

(event `/Game/BluePrints/Gamemode/BPI_Inspect.Destroy`
  (bind _bp_studio_0 (`self.BP_Studio_0`))
  (`/Engine/EditorBlueprintResources/StandardMacros.IsValid` _bp_studio_0
    (:`Is Valid`
      (`/Game/BluePrints/Gamemode/BPI_Inspect.Destroy` _bp_studio_0)
      (set `self.BP_Studio_0` null))))

(event `self.FindOtherBP_Thing.OnComponentBeginOverlap`
  (params (OverlappedComponent :type "PrimitiveComponent Object Reference") (OtherActor :type "Actor Object Reference") (OtherComp :type "PrimitiveComponent Object Reference") (OtherBodyIndex :type Integer) (bFromSweep :type Boolean) (SweepResult :type "HitResult Structure (by ref)"))
  (bind _returnvalue (`GameplayStatics.GetObjectClass` OtherActor))
  (bind _ls_shaobei (`self.LS_ShaoBei`))
  (if (== _returnvalue "/Game/BluePrints/BP_TieJiaTai.BP_TieJiaTai_C")
    (bind _aswbp_details (cast `/Game/UI/WBP_Details` (`WidgetComponent.GetUserWidgetObject` (`self.Details`))))
    (`/Game/UI/Child/WBP_Name.Set Text` (`/Game/UI/WBP_Details.WBP_Name` _aswbp_details) "装入")
    (`MovieSceneSequencePlayer.Play` (`LevelSequenceActor.SequencePlayer` (`self.LS_YuanDi`)))
    (elif (== _returnvalue "/Game/BluePrints/BP_ShaoBei.BP_ShaoBei_C")
      (bind _aswbp_details_2 (cast `/Game/UI/WBP_Details` (`WidgetComponent.GetUserWidgetObject` (`self.Details`))))
      (`/Game/UI/Child/WBP_Name.Set Text` (`/Game/UI/WBP_Details.WBP_Name` _aswbp_details_2) "倒入")
      (`LevelSequenceActor.AddBinding` _ls_shaobei (`|GetSequenceBinding` null) self false)
      (`MovieSceneSequencePlayer.Play` (`LevelSequenceActor.SequencePlayer` _ls_shaobei)))))

(event `self.FindOtherBP_Thing.OnComponentEndOverlap`
  (params (OverlappedComponent :type "PrimitiveComponent Object Reference") (OtherActor :type "Actor Object Reference") (OtherComp :type "PrimitiveComponent Object Reference") (OtherBodyIndex :type Integer))
  (bind _aswbp_details (cast `/Game/UI/WBP_Details` (`WidgetComponent.GetUserWidgetObject` (`self.Details`))))
  (`/Game/UI/Child/WBP_Name.Set Text` (`/Game/UI/WBP_Details.WBP_Name` _aswbp_details) "圆底烧瓶"))

(fn `UserConstructionScript`
  (`parent.UserConstructionScript`))

(fn `WaterHight`
  (params (Fill :type "Float (double-precision)"))
  (`parent.WaterHight` Fill))