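; BP_Door is a proximity door that swings open when the first-person character enters its Box trigger and closes when that character leaves.
; Overlap plays a timeline that drives the door mesh's yaw by the negated Rotation track; end overlap reverses it.
; Opening also plays audio, and Pawn collision is set to Block both on entry and when the timeline finishes.
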(event `self.Box.OnComponentBeginOverlap`
  (params (OverlappedComponent :type "PrimitiveComponent Object Reference") (OtherActor :type "Actor Object Reference") (OtherComp :type "PrimitiveComponent Object Reference") (OtherBodyIndex :type Integer) (bFromSweep :type Boolean) (SweepResult :type "HitResult Structure (by ref)"))
  (bind _door_sm_door_01b_lod0_001 (`self.Door_SM_Door_01b_LOD0_001`))
  (cast `/Game/Characters/FirstPerson/Blueprints/BP_FirstPersonCharacter` OtherActor)
  (`PrimitiveComponent.SetCollisionResponseToChannel` _door_sm_door_01b_lod0_001 "ECC_Pawn" "ECR_Block")
  (`AudioComponent.Play` (`self.Audio`) 0.0)
  (bind (_direction _rotation) (`Timeline|时间轴` :!label _label)
    (:`Update`
      (`SceneComponent.K2_SetRelativeRotation` (`self.Door_SM_Door_01b_LOD0_001`) (`KismetMathLibrary.MakeRotator` 0.0 0.0 (* _rotation -1.0)) false false))
    (:`Finished`
      (`PrimitiveComponent.SetCollisionResponseToChannel` _door_sm_door_01b_lod0_001 "ECC_Pawn" "ECR_Block"))))

(event `self.Box.OnComponentEndOverlap`
  (params (OverlappedComponent :type "PrimitiveComponent Object Reference") (OtherActor :type "Actor Object Reference") (OtherComp :type "PrimitiveComponent Object Reference") (OtherBodyIndex :type Integer))
  (cast `/Game/Characters/FirstPerson/Blueprints/BP_FirstPersonCharacter` OtherActor)
  (goto _label :!via `Reverse`))

(fn `UserConstructionScript`)