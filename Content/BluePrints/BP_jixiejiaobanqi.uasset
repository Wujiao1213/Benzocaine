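; Mechanical stirrer actor for a chemistry lab procedure, acting on a linked three-neck flask (BPSanJingShaoPing).
; Naming is inverted: Off starts the OFFON timeline rotating the stirrer mesh and runs two flask checks, while On stops it, gated by HasOff.
; Depending on the flask's content flags, each check waits, swaps the Niagara liquid material and calls Part2 or Part3; the latter also shows a loading widget.
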(event `self.ReceiveBeginPlay`
  (`parent.ReceiveBeginPlay`)
  (bind _returnvalue (`KismetMaterialLibrary.CreateDynamicMaterialInstance` "/Game/LiquidMaterials_VFXPack/Materials/MI_Liqui_SanJing.MI_Liqui_SanJing"))
  (set `self.WaterMaterial` _returnvalue))

(event `Off`
  (if (not (`self.HasOff`))
    (set `self.HasOff` true)
    (`self.WaterAndItem`)
    (`self.XJ And YC`)
    (bind (_direction _rotaion) (`Timeline|OFF/ON` :!label _label)
      (:`Update`
        (`SceneComponent.K2_SetRelativeRotation` (`self.机械搅拌器_搅拌器_CutPart_3E3B7250`) (`KismetMathLibrary.MakeRotator` 0.0 0.0 _rotaion) false false)))))

(event `On`
  (if (`self.HasOff`)
    (set `self.HasOff` false)
    (goto _label :!via `Stop`)))

(event `WaterAndItem`
  (bind _bp_sanjingshaoping (`self.BP_SanJingShaoPing`))
  (if (`/Game/BluePrints/BP_sanjinshaoping.HasWater` _bp_sanjingshaoping)
    (if (`/Game/BluePrints/BP_sanjinshaoping.HasItem` _bp_sanjingshaoping)
      (if (`/Game/BluePrints/BP_sanjinshaoping.HasBCS` _bp_sanjingshaoping)
        (if (not (`/Game/BluePrints/BP_sanjinshaoping.HasXJBJJYS` _bp_sanjingshaoping))
          (`KismetSystemLibrary.Delay` 3.0)
          (`NiagaraComponent.SetVariableMaterial` (`/Game/BluePrints/BP_sanjinshaoping.Water` (`self.BP_SanJingShaoPing`)) "User.Material" "/Game/LiquidMaterials_VFXPack/Materials/MI_Liqui_SanJing1.MI_Liqui_SanJing1")
          (`/Game/BluePrints/BP_sanjinshaoping.Part2` (`self.BP_SanJingShaoPing`)))))))

(event `XJ And YC`
  (bind _bp_sanjingshaoping (`self.BP_SanJingShaoPing`))
  (if (`/Game/BluePrints/BP_sanjinshaoping.HasYC` _bp_sanjingshaoping)
    (if (`/Game/BluePrints/BP_sanjinshaoping.HasXJBJJYS` _bp_sanjingshaoping)
      (bind _returnvalue (`|CreateWidget` "/Game/UI/Loading/WBP_Loading.WBP_Loading_C" (`GameplayStatics.GetPlayerController` 0)))
      (`UserWidget.AddToViewport` _returnvalue 0)
      (`KismetSystemLibrary.Delay` 3.0)
      (`NiagaraComponent.SetVariableMaterial` (`/Game/BluePrints/BP_sanjinshaoping.Water` (`self.BP_SanJingShaoPing`)) "User.Material" "/Game/LiquidMaterials_VFXPack/Materials/MI_Liqui_SanJing2.MI_Liqui_SanJing2")
      (`/Game/BluePrints/BP_sanjinshaoping.Part3` (`self.BP_SanJingShaoPing`)))))

(fn `UserConstructionScript`
  (`parent.UserConstructionScript`))