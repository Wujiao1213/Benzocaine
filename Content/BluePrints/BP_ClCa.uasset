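; BP_ClCa is the calcium chloride prop in a lab experiment, used to fill a drying tube.
; Events toggle Application visibility and play frame ranges of level sequence LSA, including cap opening, which sets CanGet.
; ThingTargeEvent plays synced prop, spoon and tube sequences if GanZaoGuan.Step1 is done, otherwise deducts points with a cotton-first tip.
; FindOtherBP_Thing overlaps toggle HasPositionUpdate.
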(event `self.ReceiveBeginPlay`
  (`parent.ReceiveBeginPlay`))

(event `DisApplication`
  (`SceneComponent.SetVisibility` (`self.Application`) false false))

(event `VisApplication`
  (`SceneComponent.SetVisibility` (`self.Application`) true false))

(event `PlayClCaAnimation`
  (bind _sequenceplayer (`LevelSequenceActor.SequencePlayer` (`self.LS_A`)))
  (`MovieSceneSequencePlayer.SetPlaybackPosition` _sequenceplayer (make `MovieSceneSequencePlaybackParams` (make `FrameTime` (make `FrameNumber` 90)) 0.0 "" "Frame" "Jump"))
  (`MovieSceneSequencePlayer.PlayTo` :`self` _sequenceplayer :`PlaybackParams` (make `MovieSceneSequencePlaybackParams` (make `FrameTime` (make `FrameNumber` 105)))))

(event `self.ThingTargeEvent`
  (bind _returnvalue (`self.GetComponentByClass` (`GameplayStatics.GetPlayerPawn` 0) "/Game/_CaiDan/_JiFen/BP/BP_JiFenZuJian.BP_JiFenZuJian_C"))
  (if (`/Game/BluePrints/BP_GanZaoGuan.Step1` (`self.GanZaoGuan`))
    (`MovieSceneSequencePlayer.SetPlaybackPosition` (`LevelSequenceActor.SequencePlayer` (`self.LS_A`)) (make `MovieSceneSequencePlaybackParams` (make `FrameTime` (make `FrameNumber` 120)) 0.0 "" "Frame" "Jump"))
    (`MovieSceneSequencePlayer.SetPlaybackPosition` (`LevelSequenceActor.SequencePlayer` (`self.LS_YaoShi`)) (make `MovieSceneSequencePlaybackParams` (make `FrameTime` (make `FrameNumber` 120)) 0.0 "" "Frame" "Jump"))
    (`MovieSceneSequencePlayer.SetPlaybackPosition` (`LevelSequenceActor.SequencePlayer` (`self.LS_GanZaoGuan`)) (make `MovieSceneSequencePlaybackParams` (make `FrameTime` (make `FrameNumber` 120)) 0.0 "" "Frame" "Jump"))
    (`MovieSceneSequencePlayer.PlayTo` :`self` (`LevelSequenceActor.SequencePlayer` (`self.LS_YaoShi`)) :`PlaybackParams` (make `MovieSceneSequencePlaybackParams` (make `FrameTime` (make `FrameNumber` 290))))
    (`MovieSceneSequencePlayer.PlayTo` :`self` (`LevelSequenceActor.SequencePlayer` (`self.LS_A`)) :`PlaybackParams` (make `MovieSceneSequencePlaybackParams` (make `FrameTime` (make `FrameNumber` 290))))
    (`MovieSceneSequencePlayer.PlayTo` :`self` (`LevelSequenceActor.SequencePlayer` (`self.LS_GanZaoGuan`)) :`PlaybackParams` (make `MovieSceneSequencePlaybackParams` (make `FrameTime` (make `FrameNumber` 290))))
    (else
      (`/Game/_CaiDan/_JiFen/BP/BP_JiFenZuJian.JianFen` _returnvalue 3)
      (`/Game/_CaiDan/_JiFen/BP/BP_JiFenZuJian.JianFenUI` _returnvalue 0 "请先装填棉花，再进行氯化钙的装填" 3 1))))

(event `RePlayClCaAnimation`
  (bind _sequenceplayer (`LevelSequenceActor.SequencePlayer` (`self.LS_A`)))
  (if (not (== (break `FrameNumber` (break `QualifiedFrameTime` (`MovieSceneSequencePlayer.GetCurrentTime` _sequenceplayer))) 120))
    (`MovieSceneSequencePlayer.SetPlaybackPosition` _sequenceplayer (make `MovieSceneSequencePlaybackParams` (make `FrameTime` (make `FrameNumber` 91)) 0.0 "" "Frame" "Jump"))
    (else
      (`MovieSceneSequencePlayer.SetPlaybackPosition` _sequenceplayer (make `MovieSceneSequencePlaybackParams` (make `FrameTime` (make `FrameNumber` 120)) 0.0 "" "Frame" "Jump"))))
  (`MovieSceneSequencePlayer.PlayTo` :`self` _sequenceplayer :`PlaybackParams` (make `MovieSceneSequencePlaybackParams` (make `FrameTime` (make `FrameNumber` 90))))
  (set `self.CanGet` false))

(event `PlayOpenCapAnimation`
  (bind _sequenceplayer (`LevelSequenceActor.SequencePlayer` (`self.LS_A`)))
  (`MovieSceneSequencePlayer.SetPlaybackPosition` _sequenceplayer (make `MovieSceneSequencePlaybackParams` (make `FrameTime` (make `FrameNumber` 105)) 0.0 "" "Frame" "Jump"))
  (`MovieSceneSequencePlayer.PlayTo` :`self` _sequenceplayer :`PlaybackParams` (make `MovieSceneSequencePlaybackParams` (make `FrameTime` (make `FrameNumber` 120))))
  (set `self.CanGet` true))

(event `self.FindOtherBP_Thing.OnComponentBeginOverlap`
  (params (OverlappedComponent :type "PrimitiveComponent Object Reference") (OtherActor :type "Actor Object Reference") (OtherComp :type "PrimitiveComponent Object Reference") (OtherBodyIndex :type Integer) (bFromSweep :type Boolean) (SweepResult :type "HitResult Structure (by ref)"))
  (set `self.HasPositionUpdate` true))

(event `self.FindOtherBP_Thing.OnComponentEndOverlap`
  (params (OverlappedComponent :type "PrimitiveComponent Object Reference") (OtherActor :type "Actor Object Reference") (OtherComp :type "PrimitiveComponent Object Reference") (OtherBodyIndex :type Integer))
  (set `self.HasPositionUpdate` false))

(fn `UserConstructionScript`
  (`parent.UserConstructionScript`))