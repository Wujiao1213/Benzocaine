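; BP_Studio is an actor that stages an item for inspection in a first-person game.
; Its Inspect event stores the target actor and copies its class into a ChildActor component to spawn a duplicate.
; It then opens WBP_Inspect with itself as parent and sets InUnableMoveUi on the player controller.
; A Destroy event removes the studio actor, while BeginPlay, overlap and Tick are unused.
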(event `/Game/BluePrints/BPI_Inspect.Inspect`
  (params (Player :type "/Game/FirstPerson/Blueprints/BP_FirstPersonCharacter Object Reference") (WhichItemToFocus :type "StaticMesh Object Reference") (ChildActor :type "Actor Object Reference"))
  (set `self.TrgetActor` ChildActor)
  (`ChildActorComponent.SetChildActorClass` (`self.ChildActor`) (`GameplayStatics.GetObjectClass` ChildActor))
  (bind _returnvalue (`|CreateWidget` "/Game/UI/WBP_Inspect.WBP_Inspect_C"))
  (bind _output_get (set `self.WBP_Inspect` _returnvalue))
  (set `/Game/UI/WBP_Inspect.ParentActor` self _output_get)
  (`UserWidget.AddToViewport` _output_get 0)
  (bind _asbp_first_person_player_control (cast `/Game/FirstPerson/Blueprints/BP_FirstPersonPlayerControl` (`GameplayStatics.GetPlayerController` 0)))
  (set `/Game/FirstPerson/Blueprints/BP_FirstPersonPlayerControl.InUnableMoveUi` true _asbp_first_person_player_control))

(event `/Game/BluePrints/BPI_Inspect.Destroy`
  (`self.K2_DestroyActor`))

(fn `UserConstructionScript`)