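; BP_JiaoTouDiGuan is a rubber-bulb dropper lab prop that reacts to the glassware it touches.
; Overlaps on FindOtherBP_Thing check the other actor's exact class and set the Details widget label to "抽取" (draw) for the 5 ml measuring cylinder or "滴取" (drip) for the round-bottom flask.
; Flask contact also plays the LSDiGuan sequence.
; Any end overlap restores the dropper's name on the label.
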(event `self.FindOtherBP_Thing.OnComponentBeginOverlap`
  (params (OverlappedComponent :type "PrimitiveComponent Object Reference") (OtherActor :type "Actor Object Reference") (OtherComp :type "PrimitiveComponent Object Reference") (OtherBodyIndex :type Integer) (bFromSweep :type Boolean) (SweepResult :type "HitResult Structure (by ref)"))
  (bind _returnvalue (`GameplayStatics.GetObjectClass` OtherActor))
  (`|ExecutionSequence`
    (:`then_0`
      (if (== _returnvalue "/Game/BluePrints/BP_LiangTong_5ml.BP_LiangTong_5ml_C")
        (bind _aswbp_details (cast `/Game/UI/WBP_Details` (`WidgetComponent.GetUserWidgetObject` (`self.Details`))))
        (`/Game/UI/Child/WBP_Name.Set Text` (`/Game/UI/WBP_Details.WBP_Name` _aswbp_details) "抽取")))
    (:`then_1`
      (if (== _returnvalue "/Game/BluePrints/BP_YuanDiShaoPing.BP_YuanDiShaoPing_C")
        (bind _aswbp_details_2 (cast `/Game/UI/WBP_Details` (`WidgetComponent.GetUserWidgetObject` (`self.Details`))))
        (`/Game/UI/Child/WBP_Name.Set Text` (`/Game/UI/WBP_Details.WBP_Name` _aswbp_details_2) "滴取")
        (`MovieSceneSequencePlayer.Play` (`LevelSequenceActor.SequencePlayer` (`self.LS_DiGuan`)))))))

(event `self.FindOtherBP_Thing.OnComponentEndOverlap`
  (params (OverlappedComponent :type "PrimitiveComponent Object Reference") (OtherActor :type "Actor Object Reference") (OtherComp :type "PrimitiveComponent Object Reference") (OtherBodyIndex :type Integer))
  (bind _aswbp_details (cast `/Game/UI/WBP_Details` (`WidgetComponent.GetUserWidgetObject` (`self.Details`))))
  (`/Game/UI/Child/WBP_Name.Set Text` (`/Game/UI/WBP_Details.WBP_Name` _aswbp_details) "胶头滴管"))

(fn `UserConstructionScript`
  (`parent.UserConstructionScript`))