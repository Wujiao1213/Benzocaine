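; Blueprint for a dry spherical (Allihn) condenser in what appears to be a chemistry lab simulation.
; ConnectionWire reveals the lower water pipe and flags the faucet as piped, or reveals the upper pipe.
; AddWater uses a timeline to scale the water mesh's height, then sets the outlet Niagara stream's flow strength.
; OffDetail sets the condenser widget's state and refreshes its view.
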(event `self.ReceiveActorBeginOverlap`
  (params (OtherActor :type "Actor Object Reference")))

(event `ConnectionWire`
  (params (`Down?` :type Boolean))
  (if `Down?`
    (`/Game/BluePrints/BP_Wire_Pipe.切换可视性` (`self.下水管`) true)
    (set `/Game/BluePrints/BP_ShuiLongTou1.HasWirePipe` true (`self.水龙头`))
    (else
      (`/Game/BluePrints/BP_Wire_Pipe.切换可视性` (`self.上水管`) true))))

(event `OffDetail`
  (params (OFF :type Boolean))
  (bind _aswbp_qiu_xing_len_ning_guan (cast `/Game/UI/Actor/WBP_QiuXingLenNingGuan` (`WidgetComponent.GetUserWidgetObject` (`self.Application`))))
  (set `/Game/UI/Actor/WBP_QiuXingLenNingGuan.state` 1 _aswbp_qiu_xing_len_ning_guan)
  (`/Game/UI/Actor/WBP_QiuXingLenNingGuan.Update View` _aswbp_qiu_xing_len_ning_guan))

(event `AddWater`
  (bind (_direction _hight) (`Timeline|Waterhigt`)
    (:`Update`
      (`SceneComponent.SetRelativeScale3D` (`self.Water`) (`KismetMathLibrary.MakeVector` 1.0 1.0 _hight)))
    (:`Finished`
      (`NiagaraComponent.SetVariableFloat` (`self.GetComponentByClass` (`self.出水管水流`) "/Script/Niagara.NiagaraComponent") "User.FlowStrength" 0.15))))

(fn `UserConstructionScript`
  (`parent.UserConstructionScript`))