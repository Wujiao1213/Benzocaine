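; BP_MianHua is a cotton item that can be added to BP_GanZaoGuan (likely a drying tube).
; Overlapping the tube switches its Details widget label from "棉花" (cotton) to "加入" (add); any end overlap restores it.
; PlayAddMianHuaToGZG plays one of two frame ranges of a shared Level Sequence, chosen by HaveContent.
; Done jumps to that range's end and hides the actor; Initial rewinds and shows it.
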(event `DestrySelf`
  (`self.K2_DestroyActor`))

(event `self.FindOtherBP_Thing.OnComponentBeginOverlap`
  (params (OverlappedComponent :type "PrimitiveComponent Object Reference") (OtherActor :type "Actor Object Reference") (OtherComp :type "PrimitiveComponent Object Reference") (OtherBodyIndex :type Integer) (bFromSweep :type Boolean) (SweepResult :type "HitResult Structure (by ref)"))
  (if (== (`GameplayStatics.GetObjectClass` OtherActor) "/Game/BluePrints/BP_GanZaoGuan.BP_GanZaoGuan_C")
    (bind _aswbp_details (cast `/Game/UI/WBP_Details` (`WidgetComponent.GetUserWidgetObject` (`self.Details`))))
    (`/Game/UI/Child/WBP_Name.Set Text` (`/Game/UI/WBP_Details.WBP_Name` _aswbp_details) "加入")))

(event `self.FindOtherBP_Thing.OnComponentEndOverlap`
  (params (OverlappedComponent :type "PrimitiveComponent Object Reference") (OtherActor :type "Actor Object Reference") (OtherComp :type "PrimitiveComponent Object Reference") (OtherBodyIndex :type Integer))
  (bind _aswbp_details (cast `/Game/UI/WBP_Details` (`WidgetComponent.GetUserWidgetObject` (`self.Details`))))
  (`/Game/UI/Child/WBP_Name.Set Text` (`/Game/UI/WBP_Details.WBP_Name` _aswbp_details) "棉花"))

(fn `Done`
  (bind _have_content (`self.Have Content`))
  (bind _sequenceplayer (`LevelSequenceActor.SequencePlayer` (`self.LS`)))
  (if (`KismetStringLibrary.EqualEqual_StrStr` _have_content "1")
    (`MovieSceneSequencePlayer.SetPlaybackPosition` _sequenceplayer (make `MovieSceneSequencePlaybackParams` (make `FrameTime` (make `FrameNumber` 95))))
    (`self.SetActorHiddenInGame` true :!label _label)
    (elif (`KismetStringLibrary.EqualEqual_StrStr` _have_content "2")
      (`MovieSceneSequencePlayer.SetPlaybackPosition` _sequenceplayer (make `MovieSceneSequencePlaybackParams` (make `FrameTime` (make `FrameNumber` 370))))
      (goto _label))))

(fn `Initial`
  (`MovieSceneSequencePlayer.SetPlaybackPosition` (`LevelSequenceActor.SequencePlayer` (`self.LS`)) (make `MovieSceneSequencePlaybackParams` (make `FrameTime` (make `FrameNumber` 0))))
  (`self.SetActorHiddenInGame` false))

(fn `Play Add MianHua To GZG`
  (bind _have_content (`self.Have Content`))
  (bind _sequenceplayer (`LevelSequenceActor.SequencePlayer` (`self.LS`)))
  (if (`KismetStringLibrary.EqualEqual_StrStr` _have_content "1")
    (`MovieSceneSequencePlayer.SetPlaybackPosition` _sequenceplayer (make `MovieSceneSequencePlaybackParams` (make `FrameTime` (make `FrameNumber` 20))))
    (`MovieSceneSequencePlayer.PlayTo` :`self` _sequenceplayer :`PlaybackParams` (make `MovieSceneSequencePlaybackParams` (make `FrameTime` (make `FrameNumber` 95))))
    (elif (`KismetStringLibrary.EqualEqual_StrStr` _have_content "2")
      (`MovieSceneSequencePlayer.SetPlaybackPosition` _sequenceplayer (make `MovieSceneSequencePlaybackParams` (make `FrameTime` (make `FrameNumber` 315))))
      (`MovieSceneSequencePlayer.PlayTo` :`self` _sequenceplayer :`PlaybackParams` (make `MovieSceneSequencePlaybackParams` (make `FrameTime` (make `FrameNumber` 370)))))))

(fn `UserConstructionScript`
  (`parent.UserConstructionScript`))