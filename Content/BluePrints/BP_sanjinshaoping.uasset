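; Three-neck flask Blueprint for a chemistry lab reduction experiment, animating each reagent addition and updating the flask's UI widget.
; Add events (water, iron powder, glacial acetic acid, ethanol and others) play frame ranges of one Level Sequence, mostly setting Has flags.
; The saturated sodium carbonate step chains into its own sequence, then resumes the main one.
; Other events update the widget or swap the water-bath liquid mesh; Init caches measuring-cylinder Niagara effects.
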(event `self.ReceiveBeginPlay`
  (`parent.ReceiveBeginPlay`)
  (`self.Init`))

(event `水体凹陷`
  (`StaticMeshComponent.SetStaticMesh` (`StaticMeshActor.StaticMeshComponent` (`self.水浴锅液体`)) "/Game/Models/Datasmith/ShuiYuGuoTi/水浴锅液体1.水浴锅液体1"))

(event `OffApplication`
  (bind _aswbp_san_jing_shao_ping (cast `/Game/UI/Actor/WBP_SanJIngShaoPing` (`WidgetComponent.GetUserWidgetObject` (`self.Application`))))
  (set `/Game/UI/Actor/WBP_SanJIngShaoPing.state` 1 _aswbp_san_jing_shao_ping)
  (`/Game/UI/Actor/WBP_SanJIngShaoPing.Update View` _aswbp_san_jing_shao_ping))

(event `continueApplication`
  (bind _aswbp_san_jing_shao_ping (cast `/Game/UI/Actor/WBP_SanJIngShaoPing` (`WidgetComponent.GetUserWidgetObject` (`self.Application`))))
  (`/Game/UI/Actor/WBP_SanJIngShaoPing.ContinuePlay` _aswbp_san_jing_shao_ping))

(event `Add35mlWater`
  (bind _sequenceplayer (`LevelSequenceActor.SequencePlayer` (`self.LS_HuanYuanFanYing`)))
  (`MovieSceneSequencePlayer.SetPlaybackPosition` _sequenceplayer (make `MovieSceneSequencePlaybackParams` (make `FrameTime` (make `FrameNumber` 90)) 0.0 "" "Frame" "Jump"))
  (`MovieSceneSequencePlayer.PlayTo` :`self` _sequenceplayer :`PlaybackParams` (make `MovieSceneSequencePlaybackParams` (make `FrameTime` (make `FrameNumber` 151))))
  (set `self.HasWater` true))

(event `AddTieFen`
  (bind _sequenceplayer (`LevelSequenceActor.SequencePlayer` (`self.LS_HuanYuanFanYing`)))
  (`MovieSceneSequencePlayer.SetPlaybackPosition` _sequenceplayer (make `MovieSceneSequencePlaybackParams` (make `FrameTime` (make `FrameNumber` 151)) 0.0 "" "Frame" "Jump"))
  (`MovieSceneSequencePlayer.PlayTo` :`self` _sequenceplayer :`PlaybackParams` (make `MovieSceneSequencePlaybackParams` (make `FrameTime` (make `FrameNumber` 192))))
  (set `self.HasItem` true))

(event `AddBingCuSuan`
  (bind _sequenceplayer (`LevelSequenceActor.SequencePlayer` (`self.LS_HuanYuanFanYing`)))
  (`MovieSceneSequencePlayer.SetPlaybackPosition` _sequenceplayer (make `MovieSceneSequencePlaybackParams` (make `FrameTime` (make `FrameNumber` 192)) 0.0 "" "Frame" "Jump"))
  (`MovieSceneSequencePlayer.PlayTo` :`self` _sequenceplayer :`PlaybackParams` (make `MovieSceneSequencePlaybackParams` (make `FrameTime` (make `FrameNumber` 253))))
  (set `self.HasBCS` true))

(event `AddXJBJJYS`
  (bind _sequenceplayer (`LevelSequenceActor.SequencePlayer` (`self.LS_HuanYuanFanYing`)))
  (`MovieSceneSequencePlayer.SetPlaybackPosition` _sequenceplayer (make `MovieSceneSequencePlaybackParams` (make `FrameTime` (make `FrameNumber` 253)) 0.0 "" "Frame" "Jump"))
  (`MovieSceneSequencePlayer.PlayTo` :`self` _sequenceplayer :`PlaybackParams` (make `MovieSceneSequencePlaybackParams` (make `FrameTime` (make `FrameNumber` 294))))
  (set `self.HasXJBJJYS` true))

(event `AddYC`
  (bind _sequenceplayer (`LevelSequenceActor.SequencePlayer` (`self.LS_HuanYuanFanYing`)))
  (`MovieSceneSequencePlayer.SetPlaybackPosition` _sequenceplayer (make `MovieSceneSequencePlaybackParams` (make `FrameTime` (make `FrameNumber` 294)) 0.0 "" "Frame" "Jump"))
  (`MovieSceneSequencePlayer.PlayTo` :`self` _sequenceplayer :`PlaybackParams` (make `MovieSceneSequencePlaybackParams` (make `FrameTime` (make `FrameNumber` 355))))
  (set `self.HasYC` true))

(event `AddPS`
  (bind _sequenceplayer (`LevelSequenceActor.SequencePlayer` (`self.LS_HuanYuanFanYing`)))
  (`MovieSceneSequencePlayer.SetPlaybackPosition` _sequenceplayer (make `MovieSceneSequencePlaybackParams` (make `FrameTime` (make `FrameNumber` 356)) 0.0 "" "Frame" "Jump"))
  (`MovieSceneSequencePlayer.PlayTo` :`self` _sequenceplayer :`PlaybackParams` (make `MovieSceneSequencePlaybackParams` (make `FrameTime` (make `FrameNumber` 398))))
  (set `self.HasPS` true))

(event `AddBHTSN`
  (bind _sequenceplayer (`LevelSequenceActor.SequencePlayer` (`self.LS_HuanYuanFanYing`)))
  (`MovieSceneSequencePlayer.SetPlaybackPosition` _sequenceplayer (make `MovieSceneSequencePlaybackParams` (make `FrameTime` (make `FrameNumber` 400)) 0.0 "" "Frame" "Jump"))
  (`MovieSceneSequencePlayer.PlayTo` :`self` _sequenceplayer :`PlaybackParams` (make `MovieSceneSequencePlaybackParams` (make `FrameTime` (make `FrameNumber` 430))))
  (add `MovieSceneSequencePlayer.OnPause` _sequenceplayer (delegate `AddBaoheTanShuanNa`)))

(event `AddBaoheTanShuanNa`
  (bind _ls_baohutansuanna (`self.LS_BaoHuTanSuanNa`))
  (`self.PlayLS` _ls_baohutansuanna 0 195)
  (add `MovieSceneSequencePlayer.OnFinished` (`LevelSequenceActor.SequencePlayer` _ls_baohutansuanna) (delegate `自定义事件`)))

(event `自定义事件`
  (`self.PlayLS` (`self.LS_HuanYuanFanYing`) 428 490))

(event `Part2`
  (bind _aswbp_san_jing_shao_ping (cast `/Game/UI/Actor/WBP_SanJIngShaoPing` (`WidgetComponent.GetUserWidgetObject` (`self.Application`))))
  (set `/Game/UI/Actor/WBP_SanJIngShaoPing.hasXiaoJi` "Visible" _aswbp_san_jing_shao_ping)
  (set `/Game/UI/Actor/WBP_SanJIngShaoPing.hasYiChun` "Visible" _aswbp_san_jing_shao_ping)
  (set `/Game/UI/Actor/WBP_SanJIngShaoPing.HasPS` "Visible" _aswbp_san_jing_shao_ping))

(event `Part3`
  (bind _aswbp_san_jing_shao_ping (cast `/Game/UI/Actor/WBP_SanJIngShaoPing` (`WidgetComponent.GetUserWidgetObject` (`self.Application`))))
  (set `/Game/UI/Actor/WBP_SanJIngShaoPing.HasGet` "Visible" _aswbp_san_jing_shao_ping)
  (set `/Game/UI/Actor/WBP_SanJIngShaoPing.HasBHTSQN` "Visible" _aswbp_san_jing_shao_ping))

(fn `Init`
  (bind _bp_liangtong (`self.BP_LiangTong`)
    (:`then`
      (for _array_element (`self.GetComponentsByTag` _bp_liangtong "/Script/Niagara.NiagaraComponent" "Water")
        (set `self.WaterElement` _array_element))
      (for _array_element_2 (`self.GetComponentsByTag` _bp_liangtong "/Script/Niagara.NiagaraComponent" "Ribbon")
        (set `self.RibbonElement` _array_element_2)))
    (:`else`)))

(fn `PlayLS`
  (params (LS :type "LevelSequenceActor Object Reference") (strat :type Integer) (end :type Integer))
  (bind _sequenceplayer (`LevelSequenceActor.SequencePlayer` LS))
  (`MovieSceneSequencePlayer.SetPlaybackPosition` _sequenceplayer (make `MovieSceneSequencePlaybackParams` (make `FrameTime` (make `FrameNumber` strat)) 0.0 "" "Frame" "Jump"))
  (`MovieSceneSequencePlayer.PlayTo` :`self` _sequenceplayer :`PlaybackParams` (make `MovieSceneSequencePlaybackParams` (make `FrameTime` (make `FrameNumber` end)))))

(fn `UserConstructionScript`
  (`parent.UserConstructionScript`))