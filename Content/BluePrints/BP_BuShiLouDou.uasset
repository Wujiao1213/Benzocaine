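; Büchner funnel actor for a lab suction-filtration interaction, paired with a WBP_BuShiLouDou widget shown through its widget component.
; Connecting the vacuum pump (ZKB) reveals the pipe and refreshes the widget.
; Adding filter paper and filtering from the flask each jump to and play their own frame range of one shared level sequence, then update widget state flags.
; A separate event re-shows the widget component.
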(event `self.ReceiveBeginPlay`
  (`parent.ReceiveBeginPlay`)
  (bind _aswbp_bu_shi_lou_dou (cast `/Game/UI/Actor/WBP_BuShiLouDou` (`WidgetComponent.GetUserWidgetObject` (`self.Application`))))
  (set `self.WBP Bu Shi Lou Dou` _aswbp_bu_shi_lou_dou))

(event `ConnectionZKB`
  (bind _wire_pipe (`self.Wire_Pipe`))
  (bind _output_get (set `/Game/BluePrints/BP_Wire_Pipe.vis` true _wire_pipe))
  (`/Game/BluePrints/BP_Wire_Pipe.切换可视性` _wire_pipe _output_get)
  (bind _aswbp_bu_shi_lou_dou (cast `/Game/UI/Actor/WBP_BuShiLouDou` (`WidgetComponent.GetUserWidgetObject` (`self.Application`))))
  (set `/Game/UI/Actor/WBP_BuShiLouDou.HasConnect` "Collapsed" _aswbp_bu_shi_lou_dou)
  (`/Game/UI/Actor/WBP_BuShiLouDou.Update View` _aswbp_bu_shi_lou_dou))

(event `ContinueWBP`
  (`SceneComponent.SetVisibility` (`self.Application`) true false))

(event `GuoLvSJSP`
  (bind _wbp_bu_shi_lou_dou (`self.WBP Bu Shi Lou Dou`))
  (bind _ls_choulv (`self.LS_ChouLV`)
    (:`then`
      (bind _sequenceplayer (`LevelSequenceActor.SequencePlayer` _ls_choulv))
      (`MovieSceneSequencePlayer.SetPlaybackPosition` _sequenceplayer (make `MovieSceneSequencePlaybackParams` (make `FrameTime` (make `FrameNumber` 32)) 0.0 "" "Frame" "Jump"))
      (`MovieSceneSequencePlayer.PlayTo` :`self` _sequenceplayer :`PlaybackParams` (make `MovieSceneSequencePlaybackParams` (make `FrameTime` (make `FrameNumber` 94))))
      (set `/Game/UI/Actor/WBP_BuShiLouDou.HasSanJingShaoPing` "Collapsed" _wbp_bu_shi_lou_dou)
      (set `/Game/UI/Actor/WBP_BuShiLouDou.HasContent` true _wbp_bu_shi_lou_dou))
    (:`else`)))

(event `AddLvZhi`
  (bind _ls_choulv (`self.LS_ChouLV`)
    (:`then`
      (bind _sequenceplayer (`LevelSequenceActor.SequencePlayer` _ls_choulv))
      (`MovieSceneSequencePlayer.SetPlaybackPosition` _sequenceplayer (make `MovieSceneSequencePlaybackParams` (make `FrameTime` (make `FrameNumber` 0)) 0.0 "" "Frame" "Jump"))
      (`MovieSceneSequencePlayer.PlayTo` :`self` _sequenceplayer :`PlaybackParams` (make `MovieSceneSequencePlaybackParams` (make `FrameTime` (make `FrameNumber` 31))))
      (set `/Game/UI/Actor/WBP_BuShiLouDou.HasLvZhi` "Collapsed" (`self.WBP Bu Shi Lou Dou`)))
    (:`else`)))

(fn `UserConstructionScript`
  (`parent.UserConstructionScript`))