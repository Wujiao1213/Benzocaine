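; BP_CiLiJiaoBanQi is the magnetic stirrer in a chemistry lab simulation, with adjustable temperature and speed.
; Clicking two child parts raises WenDu (temperature) or ZhuanSu (speed) in fixed steps and updates their display widgets.
; PlayAddWater, during the first acyl-chlorination step, checks inventory for distilled water and the required settings, then consumes it and plays a sequence segment.
; Failures show a tip in teaching mode, otherwise deduct points.
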(event `self.FindOtherBP_Thing1.OnClicked`
  (params (TouchedComponent :type "PrimitiveComponent Object Reference") (ButtonPressed :type "Key Structure"))
  (bind _output_get (set `self.WenDu` (+ (`self.WenDu`) 5)))
  (bind _aswbp_ci_li_num (cast `/Game/UI/Actor/WBP_CiLi_Num` (`WidgetComponent.GetWidget` (`self.Widget`))))
  (`/Game/UI/Actor/WBP_CiLi_Num.TextChange` _aswbp_ci_li_num _output_get))

(event `self.FindOtherBP_Thing2.OnClicked`
  (params (TouchedComponent :type "PrimitiveComponent Object Reference") (ButtonPressed :type "Key Structure"))
  (bind _output_get (set `self.ZhuanSu` (+ (`self.ZhuanSu`) 50)))
  (bind _aswbp_ci_li_num (cast `/Game/UI/Actor/WBP_CiLi_Num` (`WidgetComponent.GetWidget` (`self.Widget2`))))
  (`/Game/UI/Actor/WBP_CiLi_Num.TextChange` _aswbp_ci_li_num _output_get))

(fn `Play Add Water`
  (returns (Success :type Boolean))
  (bind _returnvalue (`GameplayStatics.GetPlayerPawn` 0))
  (bind _zhuansu (`self.ZhuanSu`))
  (bind _returnvalue_2 (`self.GetComponentByClass` _returnvalue "/Game/Characters/_KuCun/BP/BP_WanJiaKC.BP_WanJiaKC_C"))
  (bind _returnvalue_3 (`self.GetComponentByClass` _returnvalue "/Game/_CaiDan/_JiFen/BP/BP_JiFenZuJian.BP_JiFenZuJian_C"))
  (bind _sequenceplayer (`LevelSequenceActor.SequencePlayer` (`self.LS`)))
  (if (`KismetStringLibrary.EqualEqual_StrStr` (`self.Step`) "酰氯化1")
    (bind (_array_index _found) (`/Game/Characters/_KuCun/BP/BP_WanJiaKC.FindWuPinByName` _returnvalue_2 "蒸馏水"))
    (if _found
      (if (and (and (>= _zhuansu 400) (<= _zhuansu 500)) (== (`self.WenDu`) 75))
        (`/Game/Characters/_KuCun/BP/BP_WanJiaKC.Qing Chu Wu Ping by Index` _returnvalue_2 _array_index)
        (`MovieSceneSequencePlayer.SetPlaybackPosition` _sequenceplayer (make `MovieSceneSequencePlaybackParams` (make `FrameTime` (make `FrameNumber` 125))))
        (`MovieSceneSequencePlayer.PlayTo` :`self` _sequenceplayer :`PlaybackParams` (make `MovieSceneSequencePlaybackParams` (make `FrameTime` (make `FrameNumber` 280))))
        (return true)
        (else
          (bind (_moshi _is_jiaoxue) (`/Game/_CaiDan/_JiFen/BP/BP_YouXiMoShiHSK.GetMoShi`))
          (if _is_jiaoxue
            (bind _returnvalue_4 (`|CreateWidget` "/Game/UI/WBP_tips_Normal.WBP_tips_Normal_C" null (0.0 0.0 0.0) "该操作需要在75度的恒温与400到500的转速条件下"))
            (`UserWidget.AddToViewport` _returnvalue_4 0)
            (return false)
            (else
              (`/Game/_CaiDan/_JiFen/BP/BP_JiFenZuJian.JianFen` _returnvalue_3 4)
              (`/Game/_CaiDan/_JiFen/BP/BP_JiFenZuJian.JianFenUI` _returnvalue_3 0 "该操作需要在75度的恒温与400到500的转速条件下" 4 0)
              (return false)))))
      (else
        (bind (_moshi_2 _is_jiaoxue_2) (`/Game/_CaiDan/_JiFen/BP/BP_YouXiMoShiHSK.GetMoShi`))
        (if _is_jiaoxue_2
          (bind _returnvalue_5 (`|CreateWidget` "/Game/UI/WBP_tips_Normal.WBP_tips_Normal_C" null (0.0 0.0 0.0) "该操作需要在反应中加水防止烧干"))
          (`/Game/UI/WBP_tips_Normal.Set Tips Context` _returnvalue_5 "该操作需要在反应中加水防止烧干")
          (`UserWidget.AddToViewport` _returnvalue_5 0)
          (return false)
          (else
            (`/Game/_CaiDan/_JiFen/BP/BP_JiFenZuJian.JianFen` _returnvalue_3 4)
            (`/Game/_CaiDan/_JiFen/BP/BP_JiFenZuJian.JianFenUI` _returnvalue_3 0 "该操作需要在反应中加水防止烧干" 4 0)
            (return false)))))))

(fn `UserConstructionScript`
  (`parent.UserConstructionScript`))