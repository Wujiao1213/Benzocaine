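; BP_Char is a character in the ASR (speech recognition) system that opens a chat UI when the first-person character overlaps its Box.
; On overlap it registers itself with BP_FirstPersonPlayerControl, then creates WBP_ChatUI with itself as Pawn.
; A handler appends recognized text to the UI's request field.
; The start/stop events are empty, and their bindings, the recognition binding and button-state logic are disconnected, so speech input is inactive.
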(event `StartASR`
  ;[1 1 1] StartASR Button click
)

(event `self.Box.OnComponentBeginOverlap`
  (params (OverlappedComponent :type "PrimitiveComponent Object Reference") (OtherActor :type "Actor Object Reference") (OtherComp :type "PrimitiveComponent Object Reference") (OtherBodyIndex :type Integer) (bFromSweep :type Boolean) (SweepResult :type "HitResult Structure (by ref)"))
  (cast `/Game/Characters/FirstPerson/Blueprints/BP_FirstPersonCharacter` OtherActor)
  (`|ExecutionSequence`
    (:`then_0`
      (bind _asbp_first_person_player_control (cast `/Game/Characters/FirstPerson/Blueprints/BP_FirstPersonPlayerControl` (`GameplayStatics.GetPlayerController` 0)))
      (set `/Game/Characters/FirstPerson/Blueprints/BP_FirstPersonPlayerControl.BP_Char` self _asbp_first_person_player_control))
    (:`then_1`
      (bind _returnvalue (`|CreateWidget` "/Game/UI/NPC_UI/WBP_ChatUI.WBP_ChatUI_C" (`GameplayStatics.GetPlayerController` 0) self))
      (bind _output_get (set `self.UI` _returnvalue))
      (`UserWidget.AddToViewport` _output_get 0))))

(event `Stopasr_1`
  ;[1 1 1] Stop Button click
)

(event `OnTextRecognized_事件` :!signature `self.OnTextRecognized`
  (params (Text :type String) (bIsFinished :type Boolean))
  (bind _requestcontent (`/Game/UI/NPC_UI/WBP_ChatUI.RequestContent` (`self.UI`)))
  ;[1 1 1] 识别
  (set `MultiLineEditableTextBox.Text` (`KismetTextLibrary.Conv_StringToText` (`KismetStringLibrary.Concat_StrStr` (`KismetTextLibrary.Conv_TextToString` (`MultiLineEditableTextBox.Text` _requestcontent)) Text)) _requestcontent))

(event `self.ReceiveTick`
  (params (DeltaSeconds :type "Float (single-precision)")))

(fn `UserConstructionScript`)