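; Waste-liquid bucket (FeiYeTong) for what appears to be a lab simulation, playing disposal sequences based on items in the player's inventory.
; PlayFeiYe searches the BP_WanJiaKC component for a Büchner funnel and a receiving flask, playing a level sequence for each one found.
; A found flask is also selected and checked out of inventory at a fixed transform.
; That branch returns a quiz (DaTi) index, flagged true only the first time.
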(fn `Play FeiYe`
  (returns (`Have DaTi` :type Boolean) (`DaTi Index` :type Integer))
  (bind _returnvalue (`self.GetComponentByClass` (`GameplayStatics.GetPlayerPawn` 0) "/Game/Characters/_KuCun/BP/BP_WanJiaKC.BP_WanJiaKC_C"))
  (`|ExecutionSequence`
    (:`then_0`
      (bind (_array_index _found) (`/Game/Characters/_KuCun/BP/BP_WanJiaKC.FindWuPinByClass` _returnvalue "/Game/BluePrints/BP_BuShiLouDou.BP_BuShiLouDou_C"))
      (if _found
        (`self.PlayLS` (`self.LS_ChuLiFenYe`) 0 131)))
    (:`then_1`
      (bind (_array_index_2 _found_2) (`/Game/Characters/_KuCun/BP/BP_WanJiaKC.FindWuPinByClass` _returnvalue "/Game/YuWenHuang/BP_JieShouPing.BP_JieShouPing_C"))
      (if _found_2
        (`self.PlayLS` (`self.LS_JieSHouPing_FYT`) 0 200)
        (set `/Game/Characters/_KuCun/BP/BP_WanJiaKC.XuanDingIndex` _array_index_2 _returnvalue)
        (`/Game/Characters/_KuCun/BP/BP_WanJiaKC.GenXinKuCun` _returnvalue)
        (`/Game/Characters/_KuCun/BP/BP_WanJiaKC.ChuKu` :`self` _returnvalue :`Location` (65.0 33.0 165.0))
        (`|ExecutionSequence`
          (:`then_0`
            (if (not (`self.Have DaTi`))
              (set `self.Have DaTi` true)
              (return true 4)))
          (:`then_1`
            (return false 4)))))))

(fn `UserConstructionScript`
  (`parent.UserConstructionScript`))