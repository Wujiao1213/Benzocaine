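; BP_Cheng is a clickable actor with a widget component that displays a Quality number through WBP_ChengNum.
; Three box components act as buttons: Box hides the widget and Box1 shows it.
; Clicking Box2 resets Quality to zero and passes it to the widget's TextChange to update the readout.
; All logic is click-driven; BeginPlay, overlap and Tick are unused.
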(event `self.Box.OnClicked`
  (params (TouchedComponent :type "PrimitiveComponent Object Reference") (ButtonPressed :type "Key Structure"))
  (`SceneComponent.SetVisibility` (`self.Widget`) false false))

(event `self.Box1.OnClicked`
  (params (TouchedComponent :type "PrimitiveComponent Object Reference") (ButtonPressed :type "Key Structure"))
  (`SceneComponent.SetVisibility` (`self.Widget`) true false))

(event `self.Box2.OnClicked`
  (params (TouchedComponent :type "PrimitiveComponent Object Reference") (ButtonPressed :type "Key Structure"))
  (bind _output_get (set `self.quality` 0.0))
  (bind _aswbp_cheng_num (cast `/Game/UI/Actor/WBP_ChengNum` (`WidgetComponent.GetWidget` (`self.Widget`))))
  (`/Game/UI/Actor/WBP_ChengNum.TextChange` _aswbp_cheng_num _output_get))

(fn `UserConstructionScript`
  (`parent.UserConstructionScript`))