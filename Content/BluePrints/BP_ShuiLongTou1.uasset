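; BP_ShuiLongTou1 is a water faucet Blueprint that either shows running water or feeds a connected spherical condenser (BPQiuXingLenNingGuan).
; Its 开水 (turn on water) event branches on HasWirePipe: without a pipe, the OFF flag sets the Water effect's FlowStrength, with true meaning flowing.
; With a pipe, it calls AddWater on the condenser regardless of the flag and leaves the effect untouched.
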(event `开水`
  (params (OFF :type Boolean))
  (bind _water (`self.Water`))
  (if (not (`self.HasWirePipe`))
    (if OFF
      (`NiagaraComponent.SetVariableFloat` _water "User.FlowStrength" 0.15)
      (else
        (`NiagaraComponent.SetVariableFloat` _water "User.FlowStrength" 0.0)))
    (else
      (`/Game/BluePrints/BP_QiuXingLenNingGuan2.AddWater` (`self.BP_QiuXingLenNingGuan`)))))

(fn `UserConstructionScript`
  (`parent.UserConstructionScript`))