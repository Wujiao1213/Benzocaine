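; Beaker (ShaoBei) actor for a suction filtration apparatus, with a name label, liquid effect and foam mesh.
; On BeginPlay it caches the WBP_Details widget from its Details component and writes NewName into it, if set.
; AddToKuCun stores the beaker in the player pawn's BP_WanJiaKC inventory component.
; SetWaterMaterial swaps the Niagara liquid material through User.Material, and ShowPaoMo toggles the foam mesh's visibility.
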(event `self.ReceiveBeginPlay`
  (`parent.ReceiveBeginPlay`)
  (bind _aswbp_details (cast `/Game/UI/WBP_Details` (`WidgetComponent.GetUserWidgetObject` (`self.Details`))))
  (set `self.DetailsWBP` _aswbp_details)
  (`self.UpdateView`))

(event `AddToKuCun`
  (`/Game/Characters/_KuCun/BP/BP_WanJiaKC.RuKu` (`self.GetComponentByClass` (`GameplayStatics.GetPlayerPawn` 0) "/Game/Characters/_KuCun/BP/BP_WanJiaKC.BP_WanJiaKC_C") self))

(event `SetWaterMaterial`
  (params (NewMaterial :type "MaterialInterface Object Reference"))
  (`NiagaraComponent.SetVariableMaterial` (`self.Niagara`) "User.Material" NewMaterial))

(fn `ShowPaoMo`
  (`SceneComponent.ToggleVisibility` (`self.SM_PaoMo`) false))

(fn `UpdateView`
  (bind _newname (`self.NewName`))
  (if (!= _newname (`self.null`))
    (`/Game/UI/Child/WBP_Name.Set Text` (`/Game/UI/WBP_Details.WBP_Name` (`self.DetailsWBP`)) _newname)))

(fn `UserConstructionScript`
  (`parent.UserConstructionScript`))