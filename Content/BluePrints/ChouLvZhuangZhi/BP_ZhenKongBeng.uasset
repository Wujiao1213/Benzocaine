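; BP_ZhenKongBeng is a clickable vacuum pump (真空泵) actor that toggles between two states.
; Clicking the submesh flips the OFF flag and plays or reverses a timeline.
; The timeline rolls that submesh like a switch and turns the ZhiZhenSM gauge needle.
; When it finishes, material slot 7 on the pump swaps between a base material and an instance according to the flag.
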(event `self.真空泵3_Submesh_1450417C.OnClicked`
  (params (TouchedComponent :type "PrimitiveComponent Object Reference") (ButtonPressed :type "Key Structure"))
  (bind `_真空泵3` (`self.真空泵3`))
  (if (`self.OFF`)
    (set `self.OFF` false)
    (bind (_direction _yaw _zhizhen) (`Timeline|时间轴` :!via `Reverse` :!label _label)
      (:`Update`
        (`SceneComponent.K2_SetRelativeRotation` (`self.真空泵3_Submesh_1450417C`) (`KismetMathLibrary.MakeRotator` _yaw) false false)
        (`SceneComponent.K2_SetRelativeRotation` (`self.zhiZhenSM_`) (`KismetMathLibrary.MakeRotator` 90.0 _zhizhen) false false))
      (:`Finished`
        (if (`self.OFF`)
          (`PrimitiveComponent.SetMaterial` `_真空泵3` 7 "/Game/Models/Datasmith/真空泵/材质_009_Inst.材质_009_Inst")
          (else
            (`PrimitiveComponent.SetMaterial` `_真空泵3` 7 "/Game/Models/Datasmith/真空泵/材质_009.材质_009")))))
    (else
      (set `self.OFF` true)
      (goto _label))))

(fn `UserConstructionScript`)