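; BP_ChengLiangZhi is a weighing-paper actor in the suction filtration apparatus set that can be placed on a scale.
; When its FindOtherBP_Thing component overlaps a BP_Cheng scale and its LSChengLiangZhi level sequence is valid, it plays the sequence to a set frame and flags the scale's Chengliang state.
; AddToKuCun stores the actor in the player's inventory through the pawn's BP_WanJiaKC component.
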(event `self.FindOtherBP_Thing.OnComponentBeginOverlap`
  (params (OverlappedComponent :type "PrimitiveComponent Object Reference") (OtherActor :type "Actor Object Reference") (OtherComp :type "PrimitiveComponent Object Reference") (OtherBodyIndex :type Integer) (bFromSweep :type Boolean) (SweepResult :type "HitResult Structure (by ref)"))
  (if (== (`GameplayStatics.GetObjectClass` OtherActor) "/Game/BluePrints/BP_Cheng.BP_Cheng_C")
    (bind _ls_chengliangzhi (`self.LS_ChengLiangZhi`)
      (:`then`
        (`MovieSceneSequencePlayer.PlayTo` :`self` (`LevelSequenceActor.SequencePlayer` _ls_chengliangzhi) :`PlaybackParams` (make `MovieSceneSequencePlaybackParams` (make `FrameTime` (make `FrameNumber` 61))))
        (bind _asbp_cheng (cast `/Game/BluePrints/BP_Cheng` OtherActor))
        (set `/Game/BluePrints/BP_Cheng.chengliang?` true _asbp_cheng))
      (:`else`))))

(fn `Add To Ku Cun`
  (`/Game/Characters/_KuCun/BP/BP_WanJiaKC.RuKu` (`self.GetComponentByClass` (`GameplayStatics.GetPlayerPawn` 0) "/Game/Characters/_KuCun/BP/BP_WanJiaKC.BP_WanJiaKC_C") self))

(fn `UserConstructionScript`
  (`parent.UserConstructionScript`))