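; BP_Thing is an interactable world object with hover highlighting, a name label and an application widget.
; Cursor hover toggles custom depth on its static meshes and shows the Details widget, labeled with name and optional content.
; A stationary right-click on a checkable thing opens the Application widget and locks move and look input.
; Helpers turn the player's view toward LookOn via a timeline and play level sequence frame ranges.
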(event `self.ReceiveBeginPlay`
  (bind _application (`self.Application`))
  (bind _details (`self.Details`))
  (`self.SetDetailsToWidget`)
  (bind _aswbp_defult_app (cast `/Game/UI/Actor/WBP_Defult_APP` (`WidgetComponent.GetUserWidgetObject` _application))
    (:`then`
      (set `/Game/UI/Actor/WBP_Defult_APP.parent` _application _aswbp_defult_app))
    (:`CastFailed`
      _))
  (bind _aswbp_details (cast `/Game/UI/WBP_Details` (`WidgetComponent.GetUserWidgetObject` _details))
    (:`then`
      (set `/Game/UI/WBP_Details.parent` _details _aswbp_details))
    (:`CastFailed`
      _))
  (`GameplayStatics.GetActorOfClass` "/Script/LevelSequence.LevelSequenceActor"))

(event `self.OutLineMesh.OnBeginCursorOver`
  (params (TouchedComponent :type "PrimitiveComponent Object Reference"))
  (if (`self.IsCheak`)
    _
    (else
      _))
  (if (`self.OutLineReady`)
    (`self.OnOutLine`)
    (`SceneComponent.SetVisibility` (`self.Details`) true false)))

(event `self.OutLineMesh.OnEndCursorOver`
  (params (TouchedComponent :type "PrimitiveComponent Object Reference"))
  (`self.OffOutLine`)
  (`SceneComponent.SetVisibility` (`self.Details`) false false))

(event `Look For Self`
  (bind _asbp_first_person_character (cast `/Game/Characters/FirstPerson/Blueprints/BP_FirstPersonCharacter` (`GameplayStatics.GetPlayerPawn` 0)))
  (bind _output_get (set `self.StratRotation` (`Pawn.GetControlRotation` _asbp_first_person_character)))
  (set `self.Current` _output_get)
  (set `self.TargetRotation` (`KismetMathLibrary.FindLookAtRotation` (`SceneComponent.K2_GetComponentLocation` (`/Game/Characters/FirstPerson/Blueprints/BP_FirstPersonCharacter.FirstPersonCamera` _asbp_first_person_character)) (`SceneComponent.K2_GetComponentLocation` (`self.LookOn`))))
  (`Timeline|时间轴` :!via `PlayFromStart`
    (:`Update`
      (bind _output_get_2 (set `self.Current` (`KismetMathLibrary.RInterpTo` (`self.Current`) (`self.TargetRotation`) (`GameplayStatics.GetWorldDeltaSeconds`) (`self.InterpSpeed`))))
      (`Controller.SetControlRotation` (`GameplayStatics.GetPlayerController` 0) _output_get_2))))

(event `addContent`
  (params (content :type Text))
  (set `self.HasContent` true)
  (set `self.Content` content)
  (`self.SetDetailsToWidget`))

(event `self.OutLineMesh.OnClicked`
  (params (TouchedComponent :type "PrimitiveComponent Object Reference") (ButtonPressed :type "Key Structure"))
  (bind _returnvalue (`WidgetLayoutLibrary.GetMousePositionOnViewport`))
  (set `self.mousePosition` _returnvalue))

(event `self.OutLineMesh.OnReleased`
  (params (TouchedComponent :type "PrimitiveComponent Object Reference") (ButtonReleased :type "Key Structure"))
  (bind _returnvalue (`GameplayStatics.GetPlayerController` 0))
  (bind _returnvalue_2 (`WidgetLayoutLibrary.GetMousePositionOnViewport`))
  (if (== _returnvalue_2 (`self.mousePosition`))
    (if (not (`SceneComponent.bVisible` (`self.Application`)))
      (if (== ButtonReleased "RightMouseButton")
        (if (`self.IsCheak`)
          (if (not (`self.NOAPPLICATION`))
            (set `self.OutLineReady` false)
            (`SceneComponent.SetVisibility` (`self.Application`) true true)
            (`Controller.SetIgnoreMoveInput` _returnvalue true)
            (`Controller.SetIgnoreLookInput` _returnvalue true)))))))

(event `ThingTargeEvent`)

(fn `OffOutLine`
  (bind _returnvalue (`GameplayStatics.GetPlayerController` 0))
  (for _array_element (`self.K2_GetComponentsByClass` "/Script/Engine.ActorComponent")
    (bind `_as静态网格体组件` (cast `StaticMeshComponent` _array_element))
    (`PrimitiveComponent.SetRenderCustomDepth` `_as静态网格体组件` false))
  (`/Engine/EditorBlueprintResources/StandardMacros.IsValid` _returnvalue
    (:`Is Valid`
      (if (not (`Controller.IsMoveInputIgnored` _returnvalue))
        (`SceneComponent.SetVisibility` (`self.Details`) false false)
        (`SceneComponent.SetVisibility` (`self.Application`) false false)))))

(fn `OnOutLine`
  (for _array_element (`self.K2_GetComponentsByClass` "/Script/Engine.ActorComponent")
    (bind `_as静态网格体组件` (cast `StaticMeshComponent` _array_element))
    (`PrimitiveComponent.SetRenderCustomDepth` `_as静态网格体组件` true)))

(fn `PlayLS`
  (params (LS :type "LevelSequenceActor Object Reference") (Strat :type Integer) (End :type Integer))
  (bind _sequenceplayer (`LevelSequenceActor.SequencePlayer` LS))
  (`MovieSceneSequencePlayer.SetPlaybackPosition` _sequenceplayer (make `MovieSceneSequencePlaybackParams` (make `FrameTime` (make `FrameNumber` Strat))))
  (`MovieSceneSequencePlayer.PlayTo` :`self` _sequenceplayer :`PlaybackParams` (make `MovieSceneSequencePlaybackParams` (make `FrameTime` (make `FrameNumber` End)))))

(fn `SetDetailsToWidget`
  (bind _name (`self.Name`))
  (bind _aswbp_details (cast `/Game/UI/WBP_Details` (`WidgetComponent.GetUserWidgetObject` (`self.Details`))))
  (if (`self.HasContent`)
    (bind _wbp_name (`/Game/UI/WBP_Details.WBP_Name` _aswbp_details))
    (set `/Game/UI/Child/WBP_Name.Name` (`|FormatText` "{0}({1})" _name (`self.Content`)) _wbp_name)
    (else
      (set `/Game/UI/Child/WBP_Name.Name` _name _wbp_name)))
  (`/Game/UI/Child/WBP_Name.Set Text` _wbp_name ""))

(fn `UserConstructionScript`)