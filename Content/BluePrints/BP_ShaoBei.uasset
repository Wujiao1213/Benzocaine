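; BP_ShaoBei is a beaker (shao bei) actor, apparently lab equipment, that detects other objects through its FindOtherBP_Thing overlap component.
; When IsJiaoBang (likely a stirring-rod flag) is set, begin overlap stores the other actor, end overlap clears it, and both set HasPositionUpdate.
; A class check for BP_YuanDiShaoPing3 (round-bottom flask) leads to no action.
; Construction and outline on/off functions only call the parent.
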(event `self.FindOtherBP_Thing.OnComponentBeginOverlap`
  (params (OverlappedComponent :type "PrimitiveComponent Object Reference") (OtherActor :type "Actor Object Reference") (OtherComp :type "PrimitiveComponent Object Reference") (OtherBodyIndex :type Integer) (bFromSweep :type Boolean) (SweepResult :type "HitResult Structure (by ref)"))
  (`|ExecutionSequence`
    (:`then_0`
      (if (`self.IsJiaoBang`)
        (set `self.Other Actor` OtherActor)
        (set `self.HasPositionUpdate` true)))
    (:`then_1`
      (if (== (`GameplayStatics.GetObjectClass` OtherActor) "/Game/YuWenHuang/BP_YuanDiShaoPing3.BP_YuanDiShaoPing3_C")
        _))))

(event `self.FindOtherBP_Thing.OnComponentEndOverlap`
  (params (OverlappedComponent :type "PrimitiveComponent Object Reference") (OtherActor :type "Actor Object Reference") (OtherComp :type "PrimitiveComponent Object Reference") (OtherBodyIndex :type Integer))
  (if (`self.IsJiaoBang`)
    (set `self.Other Actor` null)
    (set `self.HasPositionUpdate` true)))

(fn `OffOutLine`
  (`parent.OffOutLine`))

(fn `OnOutLine`
  (`parent.OnOutLine`))

(fn `UserConstructionScript`
  (`parent.UserConstructionScript`))