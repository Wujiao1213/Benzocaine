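; BP_YaoShi is a reagent spatula (药匙) for a chemistry lab simulation, handling substances such as CaCl2 and NaOH.
; Overlaps change its label to "取用" (take) near CaCl2, play a one-shot sequence at BP_DuiXiaoJiBenJiaSuan, or trigger an open NaOH container's animation.
; Functions play frame ranges of a shared Level Sequence.
; Initial and Done jump it to content-specific frames and update WBP_YaoShi's state.
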(event `self.FindOtherBP_Thing.OnComponentBeginOverlap`
  (params (OverlappedComponent :type "PrimitiveComponent Object Reference") (OtherActor :type "Actor Object Reference") (OtherComp :type "PrimitiveComponent Object Reference") (OtherBodyIndex :type Integer) (bFromSweep :type Boolean) (SweepResult :type "HitResult Structure (by ref)"))
  (bind _sequenceplayer (`LevelSequenceActor.SequencePlayer` (`self.LS`)))
  (`|ExecutionSequence`
    (:`then_0`
      (if (== (`GameplayStatics.GetObjectClass` OtherActor) "/Game/BluePrints/BP_ClCa.BP_ClCa_C")
        (bind _aswbp_details (cast `/Game/UI/WBP_Details` (`WidgetComponent.GetUserWidgetObject` (`self.Details`))))
        (`/Game/UI/Child/WBP_Name.Set Text` (`/Game/UI/WBP_Details.WBP_Name` _aswbp_details) "取用")))
    (:`then_1`
      (if (== (`GameplayStatics.GetObjectClass` OtherActor) "/Game/BluePrints/BP_DuiXiaoJiBenJiaSuan.BP_DuiXiaoJiBenJiaSuan_C")
        (if (`self.JiHuo`)
          (set `self.JiHuo` false)
          (`MovieSceneSequencePlayer.SetPlaybackPosition` _sequenceplayer (make `MovieSceneSequencePlaybackParams` (make `FrameTime` (make `FrameNumber` 0))))
          (`MovieSceneSequencePlayer.PlayTo` :`self` _sequenceplayer :`PlaybackParams` (make `MovieSceneSequencePlaybackParams` (make `FrameTime` (make `FrameNumber` 136)))))))
    (:`then_2`
      (if (== (`GameplayStatics.GetObjectClass` OtherActor) "/Game/YuWenHuang/BP_NaOH.BP_NaOH_C")
        (bind _asbp_na_oh (cast `/Game/YuWenHuang/BP_NaOH` OtherActor))
        (if (`/Game/YuWenHuang/BP_NaOH.Open` _asbp_na_oh)
          (`/Game/YuWenHuang/BP_NaOH.Play Add NaOH` _asbp_na_oh))))))

(event `self.FindOtherBP_Thing.OnComponentEndOverlap`
  (params (OverlappedComponent :type "PrimitiveComponent Object Reference") (OtherActor :type "Actor Object Reference") (OtherComp :type "PrimitiveComponent Object Reference") (OtherBodyIndex :type Integer))
  (bind _aswbp_details (cast `/Game/UI/WBP_Details` (`WidgetComponent.GetUserWidgetObject` (`self.Details`))))
  (`/Game/UI/Child/WBP_Name.Set Text` (`/Game/UI/WBP_Details.WBP_Name` _aswbp_details) "药匙"))

(fn `Done`
  (bind _have_content (`self.Have Content`))
  (bind _sequenceplayer (`LevelSequenceActor.SequencePlayer` (`self.LS`)))
  (`|ExecutionSequence`
    (:`then_0`
      (if (`KismetStringLibrary.EqualEqual_StrStr` _have_content "CaCl2")
        (`MovieSceneSequencePlayer.SetPlaybackPosition` _sequenceplayer (make `MovieSceneSequencePlaybackParams` (make `FrameTime` (make `FrameNumber` 323)) 0.0 "" (struct) "Frame" "Jump"))))
    (:`then_1`
      (if (`KismetStringLibrary.EqualEqual_StrStr` _have_content "NaOH")
        (`MovieSceneSequencePlayer.SetPlaybackPosition` _sequenceplayer (make `MovieSceneSequencePlaybackParams` (make `FrameTime` (make `FrameNumber` 295)) 0.0 "" (struct) "Frame" "Jump"))))
    (:`then_2`
      (bind _aswbp_yao_shi (cast `/Game/YuWenHuang/WBP_YaoShi` (`WidgetComponent.GetWidget` (`self.Application`))))
      (set `/Game/YuWenHuang/WBP_YaoShi.state` 1 _aswbp_yao_shi)
      (`/Game/YuWenHuang/WBP_YaoShi.Update View` _aswbp_yao_shi))))

(fn `Initial`
  (bind _have_content (`self.Have Content`))
  (bind _sequenceplayer (`LevelSequenceActor.SequencePlayer` (`self.LS`)))
  (`|ExecutionSequence`
    (:`then_0`
      (if (`KismetStringLibrary.EqualEqual_StrStr` _have_content "CaCl2")
        (`MovieSceneSequencePlayer.SetPlaybackPosition` _sequenceplayer (make `MovieSceneSequencePlaybackParams` (make `FrameTime` (make `FrameNumber` 105)) 0.0 "" (struct) "Frame" "Jump"))))
    (:`then_1`
      (if (`KismetStringLibrary.EqualEqual_StrStr` _have_content "NaOH")
        (`MovieSceneSequencePlayer.SetPlaybackPosition` _sequenceplayer (make `MovieSceneSequencePlaybackParams` (make `FrameTime` (make `FrameNumber` -5)) 0.0 "" (struct) "Frame" "Jump"))))
    (:`then_2`
      (bind _aswbp_yao_shi (cast `/Game/YuWenHuang/WBP_YaoShi` (`WidgetComponent.GetWidget` (`self.Application`))))
      (set `/Game/YuWenHuang/WBP_YaoShi.state` 0 _aswbp_yao_shi)
      (`/Game/YuWenHuang/WBP_YaoShi.Update View` _aswbp_yao_shi))))

(fn `Play Add NaOH BLB`
  (bind _sequenceplayer (`LevelSequenceActor.SequencePlayer` (`self.LS`)))
  (`MovieSceneSequencePlayer.SetPlaybackPosition` _sequenceplayer (make `MovieSceneSequencePlaybackParams` (make `FrameTime` (make `FrameNumber` 75)) 0.0 "" (struct) "Frame" "Jump"))
  (`MovieSceneSequencePlayer.PlayTo` :`self` _sequenceplayer :`PlaybackParams` (make `MovieSceneSequencePlaybackParams` (make `FrameTime` (make `FrameNumber` 323)))))

(fn `Play CaCL`
  (bind _sequenceplayer (`LevelSequenceActor.SequencePlayer` (`self.LS`)))
  (`MovieSceneSequencePlayer.SetPlaybackPosition` _sequenceplayer (make `MovieSceneSequencePlaybackParams` (make `FrameTime` (make `FrameNumber` 105)) 0.0 "" (struct) "Frame" "Jump"))
  (`MovieSceneSequencePlayer.PlayTo` :`self` _sequenceplayer :`PlaybackParams` (make `MovieSceneSequencePlaybackParams` (make `FrameTime` (make `FrameNumber` 295)))))

(fn `UserConstructionScript`
  (`parent.UserConstructionScript`))