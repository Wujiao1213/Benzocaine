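; BP_Wire_Pipe is a spline-driven actor that builds a wire or pipe mesh along an editable spline.
; The construction script adds one spline mesh per segment, applying the configured mesh, cross-section scale and forward axis, with positions and tangents taken from adjacent spline points.
; Each piece is stored in SplineMeshListr, which 切换可视性 (toggle visibility) loops over to show or hide the run.
; BeginPlay calls that function with Vis to set initial visibility.
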(event `self.ReceiveBeginPlay`
  (`self.切换可视性` (`self.vis`)))

(event `self.ReceiveTick`
  (params (DeltaSeconds :type "Float (single-precision)")))

(fn `UserConstructionScript`
  (bind _spline (`self.Spline`))
  (bind (_meshscale_x _meshscale_y) (`KismetMathLibrary.BreakVector2D` (`self.MeshScale`)))
  (for _index (range (+ (- (`SplineComponent.GetNumberOfSplinePoints` _spline) 2) 1))
    (bind _returnvalue (`AddComponent|NODE_AddSplineMeshComponent-0`))
    (`KismetArrayLibrary.Array_Add` (`self.SplineMeshListr`) _returnvalue)
    (`StaticMeshComponent.SetStaticMesh` _returnvalue (`self.StaticMesh`))
    (`SplineMeshComponent.SetStartScale` _returnvalue (`KismetMathLibrary.MakeVector2D` _meshscale_x _meshscale_y) true)
    (`SplineMeshComponent.SetEndScale` _returnvalue (`KismetMathLibrary.MakeVector2D` _meshscale_x _meshscale_y) true)
    (`SplineMeshComponent.SetForwardAxis` _returnvalue (`self.In Forward Axis`) true)
    (bind (_location _tangent) (`SplineComponent.GetLocationAndTangentAtSplinePoint` _spline _index "Local"))
    (bind (_location_2 _tangent_2) (`SplineComponent.GetLocationAndTangentAtSplinePoint` _spline (+ _index 1) "Local"))
    (`SplineMeshComponent.SetStartAndEnd` _returnvalue _location _tangent _location_2 _tangent_2 true)))

(fn `切换可视性`
  (params (`可视` :type Boolean))
  (for _array_element (`self.SplineMeshListr`)
    (`SceneComponent.SetVisibility` _array_element `可视` false)))