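; Interactive ChongFengGui cabinet, apparently a fume hood, with a clickable light switch and a vertically sliding panel.
; A Box trigger sets a USE flag on any overlap and clears it on exit, gating both click interactions.
; Clicking the Cylinder toggles the RectLight's visibility.
; Clicking the panel mesh flips OFF to play or reverse a timeline whose High track drives the panel's relative height.
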(event `self.Cylinder.OnClicked`
  (params (TouchedComponent :type "PrimitiveComponent Object Reference") (ButtonPressed :type "Key Structure"))
  (if (`self. USE`)
    (`SceneComponent.ToggleVisibility` (`self.RectLight`) false)))

(event `self.ChongFengGui_立方体_001.OnClicked`
  (params (TouchedComponent :type "PrimitiveComponent Object Reference") (ButtonPressed :type "Key Structure"))
  (if (`self. USE`)
    (if (`self.OFF`)
      (set `self.OFF` false)
      (bind (_direction _high) (`Timeline|时间轴` :!via `Reverse` :!label _label)
        (:`Update`
          (`SceneComponent.K2_SetRelativeLocation` (`self.ChongFengGui_立方体_001`) (`KismetMathLibrary.MakeVector` 219.246012 -0.975686 _high) false false)))
      (else
        (set `self.OFF` true)
        (goto _label)))))

(event `self.Box.OnComponentBeginOverlap`
  (params (OverlappedComponent :type "PrimitiveComponent Object Reference") (OtherActor :type "Actor Object Reference") (OtherComp :type "PrimitiveComponent Object Reference") (OtherBodyIndex :type Integer) (bFromSweep :type Boolean) (SweepResult :type "HitResult Structure (by ref)"))
  (set `self. USE` true))

(event `self.Box.OnComponentEndOverlap`
  (params (OverlappedComponent :type "PrimitiveComponent Object Reference") (OtherActor :type "Actor Object Reference") (OtherComp :type "PrimitiveComponent Object Reference") (OtherBodyIndex :type Integer))
  (set `self. USE` false))

(fn `UserConstructionScript`)