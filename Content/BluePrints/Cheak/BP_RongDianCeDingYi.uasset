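; Actor Blueprint for a melting point apparatus (RongDianCeDingYi) that exposes control of its widget and camera.
; Open/Off casts the user widget object from Application to WBP_RongDianCeDingYi and forwards the open flag to its OpenOffCheak function.
; ChangeCamera calls ChangeUseCamera on the Camera reference when it is valid.
; The event graph holds only disabled default events, so all behavior runs through these two functions.
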(fn `ChangeCamera`
  (bind _camera (`self.Camera`)
    (:`then`
      (`/Game/BluePrints/BP_Camera.ChangeUseCamera` _camera))
    (:`else`)))

(fn `Open/Off`
  (params (Open :type Boolean))
  (bind _aswbp_rong_dian_ce_ding_yi (cast `/Game/UI/Actor/WBP_RongDianCeDingYi` (`WidgetComponent.GetUserWidgetObject` (`self.Application`))))
  (`/Game/UI/Actor/WBP_RongDianCeDingYi.Open/Off Cheak` _aswbp_rong_dian_ce_ding_yi Open))

(fn `UserConstructionScript`
  (`parent.UserConstructionScript`))