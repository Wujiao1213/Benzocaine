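; Round-bottom flask actor for a chemistry lab acyl chlorination experiment, animating moves, reagent additions and stand (TJT) insertion or removal.
; Each function jumps or scrubs one level sequence, LSDaJianYiQi, to a frame and plays to another, so one timeline holds every animation.
; Stand in/out picks its range from Step (酰氯化1/2), Finish and HaveContent.
; Adding DMF sets Finish, adding BinTong clears it, and adding the stir bar hides its mesh.
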(fn `Play Add ASPL`
  (bind _sequenceplayer (`LevelSequenceActor.SequencePlayer` (`self.LS DaJianYiQi`)))
  (`MovieSceneSequencePlayer.SetPlaybackPosition` _sequenceplayer (make `MovieSceneSequencePlaybackParams` (make `FrameTime` (make `FrameNumber` 35)) 0.0 "" (struct) "Frame" "Jump"))
  (`MovieSceneSequencePlayer.PlayTo` :`self` _sequenceplayer :`PlaybackParams` (make `MovieSceneSequencePlaybackParams` (make `FrameTime` (make `FrameNumber` 200)))))

(fn `Play Add BinTong`
  (bind _sequenceplayer (`LevelSequenceActor.SequencePlayer` (`self.LS DaJianYiQi`)))
  (`MovieSceneSequencePlayer.SetPlaybackPosition` _sequenceplayer (make `MovieSceneSequencePlaybackParams` (make `FrameTime` (make `FrameNumber` 95)) 0.0 "" (struct) "Frame" "Jump"))
  (`MovieSceneSequencePlayer.PlayTo` :`self` _sequenceplayer :`PlaybackParams` (make `MovieSceneSequencePlaybackParams` (make `FrameTime` (make `FrameNumber` 290))))
  (set `self.Finish` false))

(fn `Play Add CiLiJiaoBangZi`
  (bind _sequenceplayer (`LevelSequenceActor.SequencePlayer` (`self.LS DaJianYiQi`)))
  (`MovieSceneSequencePlayer.SetPlaybackPosition` _sequenceplayer (make `MovieSceneSequencePlaybackParams` (make `FrameTime` (make `FrameNumber` 204)) 0.0 "" (struct) "Frame" "Jump"))
  (`MovieSceneSequencePlayer.PlayTo` :`self` _sequenceplayer :`PlaybackParams` (make `MovieSceneSequencePlaybackParams` (make `FrameTime` (make `FrameNumber` 269))))
  (`SceneComponent.SetVisibility` (`self.CiliJiaoBanZi`) false false))

(fn `Play Add DMF`
  (bind _sequenceplayer (`LevelSequenceActor.SequencePlayer` (`self.LS DaJianYiQi`)))
  (`MovieSceneSequencePlayer.SetPlaybackPosition` _sequenceplayer (make `MovieSceneSequencePlaybackParams` (make `FrameTime` (make `FrameNumber` 491)) 0.0 "" (struct) "Frame" "Jump"))
  (`MovieSceneSequencePlayer.PlayTo` :`self` _sequenceplayer :`PlaybackParams` (make `MovieSceneSequencePlaybackParams` (make `FrameTime` (make `FrameNumber` 524))))
  (set `self.Finish` true))

(fn `Play Add SOCl2`
  (bind _sequenceplayer (`LevelSequenceActor.SequencePlayer` (`self.LS DaJianYiQi`)))
  (`MovieSceneSequencePlayer.SetPlaybackPosition` _sequenceplayer (make `MovieSceneSequencePlaybackParams` (make `FrameTime` (make `FrameNumber` 274)) 0.0 "" (struct) "Frame" "Jump"))
  (`MovieSceneSequencePlayer.PlayTo` :`self` _sequenceplayer :`PlaybackParams` (make `MovieSceneSequencePlaybackParams` (make `FrameTime` (make `FrameNumber` 486)))))

(fn `Play In TJT`
  (bind _step (`self.Step`))
  (bind _sequenceplayer (`LevelSequenceActor.SequencePlayer` (`self.LS DaJianYiQi`)))
  (if (`KismetStringLibrary.EqualEqual_StrStr` _step "酰氯化1")
    (if (`self.Finish`)
      (`MovieSceneSequencePlayer.SetPlaybackPosition` _sequenceplayer (make `MovieSceneSequencePlaybackParams` (make `FrameTime` (make `FrameNumber` 640)) 0.0 "" (struct) "Frame" "Jump"))
      (`MovieSceneSequencePlayer.PlayTo` :`self` _sequenceplayer :`PlaybackParams` (make `MovieSceneSequencePlaybackParams` (make `FrameTime` (make `FrameNumber` 536))))
      (else
        (`MovieSceneSequencePlayer.SetPlaybackPosition` _sequenceplayer (make `MovieSceneSequencePlaybackParams` (make `FrameTime` (make `FrameNumber` 755)) 0.0 "" (struct) "Frame" "Jump"))
        (`MovieSceneSequencePlayer.PlayTo` :`self` _sequenceplayer :`PlaybackParams` (make `MovieSceneSequencePlaybackParams` (make `FrameTime` (make `FrameNumber` 645))))))
    (elif (`KismetStringLibrary.EqualEqual_StrStr` _step "酰氯化2")
      (if (`self.Have Content`)
        (`MovieSceneSequencePlayer.SetPlaybackPosition` _sequenceplayer (make `MovieSceneSequencePlaybackParams` (make `FrameTime` (make `FrameNumber` 45))))
        (`MovieSceneSequencePlayer.PlayTo` :`self` _sequenceplayer :`PlaybackParams` (make `MovieSceneSequencePlaybackParams` (make `FrameTime` (make `FrameNumber` 89))))
        (else
          (`MovieSceneSequencePlayer.SetPlaybackPosition` _sequenceplayer (make `MovieSceneSequencePlaybackParams` (make `FrameTime` (make `FrameNumber` 0)) 0.0 "" (struct) "Frame" "Jump"))
          (`MovieSceneSequencePlayer.PlayTo` :`self` _sequenceplayer :`PlaybackParams` (make `MovieSceneSequencePlaybackParams` (make `FrameTime` (make `FrameNumber` 40)))))))))

(fn `Play Move Back`
  (bind _sequenceplayer (`LevelSequenceActor.SequencePlayer` (`self.LS DaJianYiQi`)))
  (`MovieSceneSequencePlayer.SetPlaybackPosition` _sequenceplayer (make `MovieSceneSequencePlaybackParams` (make `FrameTime` (make `FrameNumber` 30)) 0.0 "" (struct) "Frame" "Scrub"))
  (`MovieSceneSequencePlayer.PlayTo` :`self` _sequenceplayer :`PlaybackParams` (make `MovieSceneSequencePlaybackParams` (make `FrameTime` (make `FrameNumber` 0)))))

(fn `Play Move Forward`
  (bind _sequenceplayer (`LevelSequenceActor.SequencePlayer` (`self.LS DaJianYiQi`)))
  (`MovieSceneSequencePlayer.SetPlaybackPosition` _sequenceplayer (make `MovieSceneSequencePlaybackParams` (make `FrameTime` (make `FrameNumber` 0)) 0.0 "" (struct) "Frame" "Jump"))
  (`MovieSceneSequencePlayer.PlayTo` :`self` _sequenceplayer :`PlaybackParams` (make `MovieSceneSequencePlaybackParams` (make `FrameTime` (make `FrameNumber` 30)))))

(fn `Play Out TJT`
  (bind _step (`self.Step`))
  (bind _sequenceplayer (`LevelSequenceActor.SequencePlayer` (`self.LS DaJianYiQi`)))
  (bind _sequenceplayer_2 (`LevelSequenceActor.SequencePlayer` (`self.LS DaJianYiQi`)))
  (if (`KismetStringLibrary.EqualEqual_StrStr` _step "酰氯化1")
    (if (`self.Finish`)
      (`MovieSceneSequencePlayer.SetPlaybackPosition` _sequenceplayer (make `MovieSceneSequencePlaybackParams` (make `FrameTime` (make `FrameNumber` 530)) 0.0 "" (struct) "Frame" "Jump"))
      (`MovieSceneSequencePlayer.PlayTo` :`self` _sequenceplayer :`PlaybackParams` (make `MovieSceneSequencePlaybackParams` (make `FrameTime` (make `FrameNumber` 640))))
      (else
        (`MovieSceneSequencePlayer.SetPlaybackPosition` _sequenceplayer (make `MovieSceneSequencePlaybackParams` (make `FrameTime` (make `FrameNumber` 645)) 0.0 "" (struct) "Frame" "Jump"))
        (`MovieSceneSequencePlayer.PlayTo` :`self` _sequenceplayer :`PlaybackParams` (make `MovieSceneSequencePlaybackParams` (make `FrameTime` (make `FrameNumber` 755))))))
    (elif (`KismetStringLibrary.EqualEqual_StrStr` _step "酰氯化2")
      (if (`self.Finish`)
        (`MovieSceneSequencePlayer.SetPlaybackPosition` _sequenceplayer (make `MovieSceneSequencePlaybackParams` (make `FrameTime` (make `FrameNumber` 40)) 0.0 "" (struct) "Frame" "Jump"))
        (`MovieSceneSequencePlayer.PlayTo` :`self` _sequenceplayer :`PlaybackParams` (make `MovieSceneSequencePlaybackParams` (make `FrameTime` (make `FrameNumber` 0))))
        (elif (`self.Have Content`)
          (`MovieSceneSequencePlayer.SetPlaybackPosition` _sequenceplayer_2 (make `MovieSceneSequencePlaybackParams` (make `FrameTime` (make `FrameNumber` 89)) 0.0 "" (struct) "Frame" "Jump"))
          (`MovieSceneSequencePlayer.PlayTo` :`self` _sequenceplayer_2 :`PlaybackParams` (make `MovieSceneSequencePlaybackParams` (make `FrameTime` (make `FrameNumber` 51))))
          (else
            (`MovieSceneSequencePlayer.SetPlaybackPosition` _sequenceplayer_2 (make `MovieSceneSequencePlaybackParams` (make `FrameTime` (make `FrameNumber` 40)) 0.0 "" (struct) "Frame" "Jump"))
            (`MovieSceneSequencePlayer.PlayTo` :`self` _sequenceplayer_2 :`PlaybackParams` (make `MovieSceneSequencePlaybackParams` (make `FrameTime` (make `FrameNumber` 0))))))))))

(fn `UserConstructionScript`
  (`parent.UserConstructionScript`))