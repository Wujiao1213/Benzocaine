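; Vacuum pump (ZhenKongBen) switch actor that shows the switch being opened or shut.
; PlaySwitchOpen and PlaySwitchShut each snap OutLineMesh to a fixed world rotation while keeping its location.
; Each then jumps the LS0 level sequence to a hard-coded frame and plays to an end frame, so one sequence serves both animations.
; The event graph holds only disabled default events, so both functions rely on outside callers.
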(fn `Play Switch Open`
  (bind _outlinemesh (`self.OutLineMesh`))
  (bind _sequenceplayer (`LevelSequenceActor.SequencePlayer` (`self.LS_0`)))
  (`SceneComponent.K2_SetWorldLocationAndRotation` _outlinemesh (`SceneComponent.K2_GetComponentLocation` _outlinemesh) (struct :`Roll` 70.0) false false)
  (`MovieSceneSequencePlayer.SetPlaybackPosition` _sequenceplayer (make `MovieSceneSequencePlaybackParams` (make `FrameTime` (make `FrameNumber` 355))))
  (`MovieSceneSequencePlayer.PlayTo` :`self` _sequenceplayer :`PlaybackParams` (make `MovieSceneSequencePlaybackParams` (make `FrameTime` (make `FrameNumber` 385)))))

(fn `Play Switch Shut`
  (bind _outlinemesh (`self.OutLineMesh`))
  (bind _sequenceplayer (`LevelSequenceActor.SequencePlayer` (`self.LS_0`)))
  (`SceneComponent.K2_SetWorldLocationAndRotation` _outlinemesh (`SceneComponent.K2_GetComponentLocation` _outlinemesh) (struct :`Roll` -20.0) false false)
  (`MovieSceneSequencePlayer.SetPlaybackPosition` _sequenceplayer (make `MovieSceneSequencePlaybackParams` (make `FrameTime` (make `FrameNumber` 380))))
  (`MovieSceneSequencePlayer.PlayTo` :`self` _sequenceplayer :`PlaybackParams` (make `MovieSceneSequencePlaybackParams` (make `FrameTime` (make `FrameNumber` 400)))))

(fn `UserConstructionScript`
  (`parent.UserConstructionScript`))