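; BP_SOCl is an SOCl reagent actor, apparently for a chemistry experiment, that plays use, open, add and put-back animations.
; Each action seeks and plays a frame range of one Level Sequence, LSNaOH, whose naming the functions share.
; An Open flag gates use, open and put-back; opening sets it, while adding or putting back clears it.
; Events toggle the Application component's visibility, and put-back hides it when open.
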(event `self.ReceiveBeginPlay`
  (`parent.ReceiveBeginPlay`))

(event `DisApplication`
  (`SceneComponent.SetVisibility` (`self.Application`) false false))

(event `VisApplication`
  (`SceneComponent.SetVisibility` (`self.Application`) true false))

(event `Play Back NaOH`
  (bind _sequenceplayer (`LevelSequenceActor.SequencePlayer` (`self.LS_NaOH`)))
  (if (`self.Open`)
    (`MovieSceneSequencePlayer.SetPlaybackPosition` _sequenceplayer (make `MovieSceneSequencePlaybackParams` (make `FrameTime` (make `FrameNumber` 293))))
    (`MovieSceneSequencePlayer.PlayTo` :`self` _sequenceplayer :`PlaybackParams` (make `MovieSceneSequencePlaybackParams` (make `FrameTime` (make `FrameNumber` 323))))
    (set `self.Open` false)
    (`SceneComponent.SetVisibility` (`self.Application`) false false)
    (else
      (`MovieSceneSequencePlayer.SetPlaybackPosition` _sequenceplayer (make `MovieSceneSequencePlaybackParams` (make `FrameTime` (make `FrameNumber` 0)) 0.0 "" (struct) "Frame" "Jump")))))

(event `Play Open SOCl`
  (bind _sequenceplayer (`LevelSequenceActor.SequencePlayer` (`self.LS_NaOH`)))
  (if (not (`self.Open`))
    (`MovieSceneSequencePlayer.SetPlaybackPosition` _sequenceplayer (make `MovieSceneSequencePlaybackParams` (make `FrameTime` (make `FrameNumber` 45)) 0.0 "" (struct) "Frame" "Jump"))
    (`MovieSceneSequencePlayer.PlayTo` :`self` _sequenceplayer :`PlaybackParams` (make `MovieSceneSequencePlaybackParams` (make `FrameTime` (make `FrameNumber` 75))))
    (set `self.Open` true)))

(fn `Chen Liang`)

(fn `Play Add NaOH`
  (bind _sequenceplayer (`LevelSequenceActor.SequencePlayer` (`self.LS_NaOH`)))
  (`MovieSceneSequencePlayer.SetPlaybackPosition` _sequenceplayer (make `MovieSceneSequencePlaybackParams` (make `FrameTime` (make `FrameNumber` 75)) 0.0 "" (struct) "Frame" "Jump"))
  (`MovieSceneSequencePlayer.PlayTo` :`self` _sequenceplayer :`PlaybackParams` (make `MovieSceneSequencePlaybackParams` (make `FrameTime` (make `FrameNumber` 323))))
  (set `self.Open` false))

(fn `Play Use NaOH`
  (bind _sequenceplayer (`LevelSequenceActor.SequencePlayer` (`self.LS_NaOH`)))
  (if (not (`self.Open`))
    (`MovieSceneSequencePlayer.SetPlaybackPosition` _sequenceplayer (make `MovieSceneSequencePlaybackParams` (make `FrameTime` (make `FrameNumber` 0)) 0.0 "" (struct) "Frame" "Jump"))
    (`MovieSceneSequencePlayer.PlayTo` :`self` _sequenceplayer :`PlaybackParams` (make `MovieSceneSequencePlaybackParams` (make `FrameTime` (make `FrameNumber` 44))))))

(fn `UserConstructionScript`
  (`parent.UserConstructionScript`))