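; Spherical condenser (QiuXingLengNingGuan) actor for what appears to be a lab simulation, with water hoses, a faucet link and an iron stand (TJT).
; ConnectionWire shows the lower or upper hose, flagging the faucet as piped for the lower one.
; AddWater scales the water mesh up by timeline, then sets the outlet Niagara flow.
; Helpers play frame ranges of one level sequence for stand and pipe moves; OffDetail refreshes the condenser widget.
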(event `self.ReceiveActorBeginOverlap`
  (params (OtherActor :type "Actor Object Reference")))

(event `ConnectionWire`
  (params (`Down?` :type Boolean))
  (if `Down?`
    (`/Game/BluePrints/BP_Wire_Pipe.切换可视性` (`self.下水管`) true)
    (set `/Game/BluePrints/BP_ShuiLongTou1.HasWirePipe` true (`self.水龙头`))
    (else
      (`/Game/BluePrints/BP_Wire_Pipe.切换可视性` (`self.上水管`) true))))

(event `OffDetail`
  (params (OFF :type Boolean))
  (bind _aswbp_qiu_xing_len_ning_guan (cast `/Game/UI/Actor/WBP_QiuXingLenNingGuan` (`WidgetComponent.GetUserWidgetObject` (`self.Application`))))
  (set `/Game/UI/Actor/WBP_QiuXingLenNingGuan.state` 1 _aswbp_qiu_xing_len_ning_guan)
  (`/Game/UI/Actor/WBP_QiuXingLenNingGuan.Update View` _aswbp_qiu_xing_len_ning_guan))

(event `AddWater`
  (bind (_direction _hight) (`Timeline|Waterhigt`)
    (:`Update`
      (`SceneComponent.SetRelativeScale3D` (`self.Water`) (`KismetMathLibrary.MakeVector` 1.0 1.0 _hight)))
    (:`Finished`
      (`NiagaraComponent.SetVariableFloat` (`self.GetComponentByClass` (`self.出水管水流`) "/Script/Niagara.NiagaraComponent") "User.FlowStrength" 0.15))))

(event `self.FindOtherBP_Thing.OnComponentBeginOverlap`
  (params (OverlappedComponent :type "PrimitiveComponent Object Reference") (OtherActor :type "Actor Object Reference") (OtherComp :type "PrimitiveComponent Object Reference") (OtherBodyIndex :type Integer) (bFromSweep :type Boolean) (SweepResult :type "HitResult Structure (by ref)"))
  (if (== (`GameplayStatics.GetObjectClass` OtherActor) "/Game/YuWenHuang/BP_TieJiaTai_Zu0.BP_TieJiaTai_Zu0_C")
    (cast `/Game/YuWenHuang/BP_TieJiaTai_Zu0` OtherActor)
    (set `self.BP_TJT` null)))

(fn `Play Move In TJT`
  (bind _sequenceplayer (`LevelSequenceActor.SequencePlayer` (`self.LS_TJT`)))
  (`MovieSceneSequencePlayer.SetPlaybackPosition` _sequenceplayer (make `MovieSceneSequencePlaybackParams` (make `FrameTime` (make `FrameNumber` 0))))
  (`MovieSceneSequencePlayer.PlayTo` :`self` _sequenceplayer :`PlaybackParams` (make `MovieSceneSequencePlaybackParams` (make `FrameTime` (make `FrameNumber` 55)))))

(fn `Play Move Out TJT`
  (bind _sequenceplayer (`LevelSequenceActor.SequencePlayer` (`self.LS_TJT`)))
  (`MovieSceneSequencePlayer.SetPlaybackPosition` _sequenceplayer (make `MovieSceneSequencePlaybackParams` (make `FrameTime` (make `FrameNumber` 55))))
  (`MovieSceneSequencePlayer.PlayTo` :`self` _sequenceplayer :`PlaybackParams` (make `MovieSceneSequencePlaybackParams` (make `FrameTime` (make `FrameNumber` 0)))))

(fn `Play Pipe Down To Up`
  (bind _sequenceplayer (`LevelSequenceActor.SequencePlayer` (`self.LS_TJT`)))
  (`MovieSceneSequencePlayer.SetPlaybackPosition` _sequenceplayer (make `MovieSceneSequencePlaybackParams` (make `FrameTime` (make `FrameNumber` 65))))
  (`MovieSceneSequencePlayer.PlayTo` :`self` _sequenceplayer :`PlaybackParams` (make `MovieSceneSequencePlaybackParams` (make `FrameTime` (make `FrameNumber` 130)))))

(fn `UserConstructionScript`
  (`parent.UserConstructionScript`))