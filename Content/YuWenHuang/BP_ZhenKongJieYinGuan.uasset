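; Blueprint for a vacuum adapter tube (ZhenKongJieYinGuan), apparently lab apparatus, that exposes functions to animate it moving in and out and its pipe being added or removed.
; Each function jumps the sequence player of LS to a fixed frame, then plays to another.
; Paired actions reuse the same frame range with endpoints swapped, so one animation serves both directions.
; The event graph is inactive, leaving these functions to be triggered externally.
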(fn `Play Add Pipe`
  (bind _sequenceplayer (`LevelSequenceActor.SequencePlayer` (`self.LS`)))
  (`MovieSceneSequencePlayer.SetPlaybackPosition` _sequenceplayer (make `MovieSceneSequencePlaybackParams` (make `FrameTime` (make `FrameNumber` 310))))
  (`MovieSceneSequencePlayer.PlayTo` :`self` _sequenceplayer :`PlaybackParams` (make `MovieSceneSequencePlaybackParams` (make `FrameTime` (make `FrameNumber` 360)))))

(fn `Play Move In Pipe`
  (bind _sequenceplayer (`LevelSequenceActor.SequencePlayer` (`self.LS`)))
  (`MovieSceneSequencePlayer.SetPlaybackPosition` _sequenceplayer (make `MovieSceneSequencePlaybackParams` (make `FrameTime` (make `FrameNumber` 449))))
  (`MovieSceneSequencePlayer.PlayTo` :`self` _sequenceplayer :`PlaybackParams` (make `MovieSceneSequencePlaybackParams` (make `FrameTime` (make `FrameNumber` 425)))))

(fn `Play Move In TJT`
  (bind _sequenceplayer (`LevelSequenceActor.SequencePlayer` (`self.LS`)))
  (`MovieSceneSequencePlayer.SetPlaybackPosition` _sequenceplayer (make `MovieSceneSequencePlaybackParams` (make `FrameTime` (make `FrameNumber` 285))))
  (`MovieSceneSequencePlayer.PlayTo` :`self` _sequenceplayer :`PlaybackParams` (make `MovieSceneSequencePlaybackParams` (make `FrameTime` (make `FrameNumber` 315)))))

(fn `Play Move Out Pipe`
  (bind _sequenceplayer (`LevelSequenceActor.SequencePlayer` (`self.LS`)))
  (`MovieSceneSequencePlayer.SetPlaybackPosition` _sequenceplayer (make `MovieSceneSequencePlaybackParams` (make `FrameTime` (make `FrameNumber` 425))))
  (`MovieSceneSequencePlayer.PlayTo` :`self` _sequenceplayer :`PlaybackParams` (make `MovieSceneSequencePlaybackParams` (make `FrameTime` (make `FrameNumber` 449)))))

(fn `Play Move Out TJT`
  (bind _sequenceplayer (`LevelSequenceActor.SequencePlayer` (`self.LS`)))
  (`MovieSceneSequencePlayer.SetPlaybackPosition` _sequenceplayer (make `MovieSceneSequencePlaybackParams` (make `FrameTime` (make `FrameNumber` 315))))
  (`MovieSceneSequencePlayer.PlayTo` :`self` _sequenceplayer :`PlaybackParams` (make `MovieSceneSequencePlaybackParams` (make `FrameTime` (make `FrameNumber` 285)))))

(fn `Play Remove Pipe`
  (bind _sequenceplayer (`LevelSequenceActor.SequencePlayer` (`self.LS`)))
  (`MovieSceneSequencePlayer.SetPlaybackPosition` _sequenceplayer (make `MovieSceneSequencePlaybackParams` (make `FrameTime` (make `FrameNumber` 360))))
  (`MovieSceneSequencePlayer.PlayTo` :`self` _sequenceplayer :`PlaybackParams` (make `MovieSceneSequencePlaybackParams` (make `FrameTime` (make `FrameNumber` 310)))))

(fn `UserConstructionScript`
  (`parent.UserConstructionScript`))