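; BP_PuReXiTong is an interactive Blueprint actor that drives sodium hydroxide (NaOH) animations through the LSNaOH level sequence.
; PlayUseNaOH plays the opening segment only while Open is false, and PlayAddNaOH plays a later segment, then clears Open.
; Both jump the sequence player to a frame and use PlayTo, so one sequence holds both actions.
; The FindOtherBP_Thing overlap events and ChenLiang function are empty stubs.
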(event `self.ReceiveBeginPlay`
  (`parent.ReceiveBeginPlay`))

(event `self.FindOtherBP_Thing.OnComponentBeginOverlap`
  (params (OverlappedComponent :type "PrimitiveComponent Object Reference") (OtherActor :type "Actor Object Reference") (OtherComp :type "PrimitiveComponent Object Reference") (OtherBodyIndex :type Integer) (bFromSweep :type Boolean) (SweepResult :type "HitResult Structure (by ref)")))

(event `self.FindOtherBP_Thing.OnComponentEndOverlap`
  (params (OverlappedComponent :type "PrimitiveComponent Object Reference") (OtherActor :type "Actor Object Reference") (OtherComp :type "PrimitiveComponent Object Reference") (OtherBodyIndex :type Integer)))

(fn `Chen Liang`)

(fn `Play Add NaOH`
  (bind _sequenceplayer (`LevelSequenceActor.SequencePlayer` (`self.LS_NaOH`)))
  (`MovieSceneSequencePlayer.SetPlaybackPosition` _sequenceplayer (make `MovieSceneSequencePlaybackParams` (make `FrameTime` (make `FrameNumber` 75)) 0.0 "" (struct) "Frame" "Jump"))
  (`MovieSceneSequencePlayer.PlayTo` :`self` _sequenceplayer :`PlaybackParams` (make `MovieSceneSequencePlaybackParams` (make `FrameTime` (make `FrameNumber` 323))))
  (set `self.Open` false))

(fn `Play Use NaOH`
  (bind _sequenceplayer (`LevelSequenceActor.SequencePlayer` (`self.LS_NaOH`)))
  (if (not (`self.Open`))
    (`MovieSceneSequencePlayer.SetPlaybackPosition` _sequenceplayer (make `MovieSceneSequencePlaybackParams` (make `FrameTime` (make `FrameNumber` 0)) 0.0 "" (struct) "Frame" "Jump"))
    (`MovieSceneSequencePlayer.PlayTo` :`self` _sequenceplayer :`PlaybackParams` (make `MovieSceneSequencePlaybackParams` (make `FrameTime` (make `FrameNumber` 44))))))

(fn `UserConstructionScript`
  (`parent.UserConstructionScript`))