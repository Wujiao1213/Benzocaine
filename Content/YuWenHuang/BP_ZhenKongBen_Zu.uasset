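; Vacuum pump group actor for what appears to be a lab experiment simulation, playing the pump switch's open and shut animations.
; Each action rotates the switch and plays its own frame range of a shared Level Sequence.
; Opening is unconditional with an empty flask; otherwise the first magnetic stirrer found must read 60–70 temperature, or it fails and reports whether teaching mode is active.
; Loops passing the sequence to child switches are unconnected.
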(fn `Play Switch Open`
  (returns (`Is JiaoXue` :type Boolean) (Success :type Boolean))
  (bind _bp_zhenkongben_switch (`self.BP_ZhenKongBen_Switch`))
  (bind _sequenceplayer (`LevelSequenceActor.SequencePlayer` (`self.LS_Switch`)))
  (if (`/Game/YuWenHuang/BP_YuanDiShaoPing3.Have Content` (`self.BP_ShaoPing`))
    (for _array_element (`SceneComponent.GetChildrenComponents` (`/Game/YuWenHuang/BP_TieJiaTai_Zu.BP_CiLiJiaoBanQi` (`self.BP_TieJiaTaiZu`)) true)
      (bind _asbp_ci_li_jiao_ban_qi (cast `/Game/BluePrints/BP_CiLiJiaoBanQi` (`ActorComponent.GetOwner` _array_element)))
      (bind _wendu (`/Game/BluePrints/BP_CiLiJiaoBanQi.WenDu` _asbp_ci_li_jiao_ban_qi))
      (if (and (>= _wendu 60) (<= _wendu 70))
        (`SceneComponent.K2_SetWorldLocationAndRotation` _bp_zhenkongben_switch (`SceneComponent.K2_GetComponentLocation` _bp_zhenkongben_switch) (struct :`Roll` 70.0) false false :!label _label)
        (`MovieSceneSequencePlayer.SetPlaybackPosition` _sequenceplayer (make `MovieSceneSequencePlaybackParams` (make `FrameTime` (make `FrameNumber` 355)) 0.0 "" (struct) "Frame" "Jump"))
        (`MovieSceneSequencePlayer.PlayTo` :`self` _sequenceplayer :`PlaybackParams` (make `MovieSceneSequencePlaybackParams` (make `FrameTime` (make `FrameNumber` 424))))
        (return false true)
        (else
          (bind (_moshi _is_jiaoxue) (`/Game/_CaiDan/_JiFen/BP/BP_YouXiMoShiHSK.GetMoShi`))
          (if _is_jiaoxue
            (return true false)
            (else
              (return false false))))))
    (else
      (goto _label))))

(fn `Play Switch Shut`
  (bind _bp_zhenkongben_switch (`self.BP_ZhenKongBen_Switch`))
  (bind _sequenceplayer (`LevelSequenceActor.SequencePlayer` (`self.LS_Switch`)))
  (`SceneComponent.K2_SetWorldLocationAndRotation` _bp_zhenkongben_switch (`SceneComponent.K2_GetComponentLocation` _bp_zhenkongben_switch) (struct :`Roll` -20.0) false false)
  (`MovieSceneSequencePlayer.SetPlaybackPosition` _sequenceplayer (make `MovieSceneSequencePlaybackParams` (make `FrameTime` (make `FrameNumber` 450)) 0.0 "" (struct) "Frame" "Jump"))
  (`MovieSceneSequencePlayer.PlayTo` :`self` _sequenceplayer :`PlaybackParams` (make `MovieSceneSequencePlaybackParams` (make `FrameTime` (make `FrameNumber` 489)))))

(fn `UserConstructionScript`
  (`parent.UserConstructionScript`))