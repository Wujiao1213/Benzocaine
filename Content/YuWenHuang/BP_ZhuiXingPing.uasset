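; BP_ZhuiXingPing is a conical flask Blueprint that plays two-step transport animations and tracks whether it has content.
; PlayTransportResult branches on Step, driving level sequence players with SetPlaybackPosition and PlayTo frame targets.
; Outside step 2, it runs LSStep1 to a frame, advances to step 2 and sets HaveContent.
; At step 2, it calls Play on LSStep1, runs LSStep2 to a frame and clears HaveContent.
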(event `self.ReceiveBeginPlay`
  (`parent.ReceiveBeginPlay`))

(fn `Play Transport Result`
  (bind _sequenceplayer (`LevelSequenceActor.SequencePlayer` (`self.LS_Step2`)))
  (bind _sequenceplayer_2 (`LevelSequenceActor.SequencePlayer` (`self.LS_Step1`)))
  (if (== (`self.Step`) 2)
    (`MovieSceneSequencePlayer.Play` _sequenceplayer_2)
    (`MovieSceneSequencePlayer.SetPlaybackPosition` _sequenceplayer (make `MovieSceneSequencePlaybackParams` (make `FrameTime` (make `FrameNumber` 0))))
    (`MovieSceneSequencePlayer.PlayTo` :`self` _sequenceplayer :`PlaybackParams` (make `MovieSceneSequencePlaybackParams` (make `FrameTime` (make `FrameNumber` 165))))
    (set `self.Have Content` false)
    (else
      (`MovieSceneSequencePlayer.SetPlaybackPosition` _sequenceplayer_2 (make `MovieSceneSequencePlaybackParams` (make `FrameTime` (make `FrameNumber` 0))))
      (`MovieSceneSequencePlayer.PlayTo` :`self` _sequenceplayer_2 :`PlaybackParams` (make `MovieSceneSequencePlaybackParams` (make `FrameTime` (make `FrameNumber` 260))))
      (set `self.Step` 2)
      (set `self.Have Content` true))))

(fn `UserConstructionScript`
  (`parent.UserConstructionScript`))