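; Water basin (ShuiPeng) actor that can be filled, emptied, inspected and moved in and out of an iron stand (TieJiaTai).
; Functions play frame ranges of one level sequence forward or backward; the water ones also set HaveWater.
; CheakActor spawns a far-off BP_Studio to inspect the basin, and Destroy removes that studio.
; Ending overlap resets the Details widget name; begin overlap checks for the stand but does nothing.
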(event `CheakActor`
  (bind _returnvalue (`|SpawnActorFromClass` "/Game/BluePrints/BP_Studio.BP_Studio_C" (`KismetMathLibrary.MakeTransform` (100000000.0 0.0 0.0)) "Undefined" "MultiplyWithRoot" null null))
  (bind _output_get (set `self.BP_Studio_0` _returnvalue))
  (`/Game/BluePrints/Gamemode/BPI_Inspect.Inspect` _output_get null null self))

(event `self.Destroy`
  (bind _bp_studio_0 (`self.BP_Studio_0`))
  (`/Engine/EditorBlueprintResources/StandardMacros.IsValid` _bp_studio_0
    (:`Is Valid`
      (`/Game/BluePrints/Gamemode/BPI_Inspect.Destroy` _bp_studio_0)
      (set `self.BP_Studio_0` null))))

(event `self.FindOtherBP_Thing.OnComponentBeginOverlap`
  (params (OverlappedComponent :type "PrimitiveComponent Object Reference") (OtherActor :type "Actor Object Reference") (OtherComp :type "PrimitiveComponent Object Reference") (OtherBodyIndex :type Integer) (bFromSweep :type Boolean) (SweepResult :type "HitResult Structure (by ref)"))
  (if (== (`GameplayStatics.GetObjectClass` OtherActor) "/Game/YuWenHuang/BP_TieJiaTai_Zu0.BP_TieJiaTai_Zu0_C")
    _))

(event `self.FindOtherBP_Thing.OnComponentEndOverlap`
  (params (OverlappedComponent :type "PrimitiveComponent Object Reference") (OtherActor :type "Actor Object Reference") (OtherComp :type "PrimitiveComponent Object Reference") (OtherBodyIndex :type Integer))
  (bind _aswbp_details (cast `/Game/UI/WBP_Details` (`WidgetComponent.GetUserWidgetObject` (`self.Details`))))
  (`/Game/UI/Child/WBP_Name.Set Text` (`/Game/UI/WBP_Details.WBP_Name` _aswbp_details) "装入水的水盆"))

(fn `Play Add Water`
  (bind _sequenceplayer (`LevelSequenceActor.SequencePlayer` (`self.LS_ShuiPeng`)))
  (`MovieSceneSequencePlayer.SetPlaybackPosition` _sequenceplayer (make `MovieSceneSequencePlaybackParams` (make `FrameTime` (make `FrameNumber` 0)) 0.0 "" (struct) "Frame" "Jump"))
  (`MovieSceneSequencePlayer.PlayTo` :`self` _sequenceplayer :`PlaybackParams` (make `MovieSceneSequencePlaybackParams` (make `FrameTime` (make `FrameNumber` 60))))
  (set `self.Have Water` true))

(fn `Play Move In TJT`
  (bind _sequenceplayer (`LevelSequenceActor.SequencePlayer` (`self.LS_ShuiPeng`)))
  (`MovieSceneSequencePlayer.SetPlaybackPosition` _sequenceplayer (make `MovieSceneSequencePlaybackParams` (make `FrameTime` (make `FrameNumber` 65)) 0.0 "" (struct) "Frame" "Jump"))
  (`MovieSceneSequencePlayer.PlayTo` :`self` _sequenceplayer :`PlaybackParams` (make `MovieSceneSequencePlaybackParams` (make `FrameTime` (make `FrameNumber` 126)))))

(fn `Play Move Out TJT`
  (bind _sequenceplayer (`LevelSequenceActor.SequencePlayer` (`self.LS_ShuiPeng`)))
  (`MovieSceneSequencePlayer.SetPlaybackPosition` _sequenceplayer (make `MovieSceneSequencePlaybackParams` (make `FrameTime` (make `FrameNumber` 126))))
  (`MovieSceneSequencePlayer.PlayTo` :`self` _sequenceplayer :`PlaybackParams` (make `MovieSceneSequencePlaybackParams` (make `FrameTime` (make `FrameNumber` 65)))))

(fn `Play Remove Water`
  (bind _sequenceplayer (`LevelSequenceActor.SequencePlayer` (`self.LS_ShuiPeng`)))
  (`MovieSceneSequencePlayer.SetPlaybackPosition` _sequenceplayer (make `MovieSceneSequencePlaybackParams` (make `FrameTime` (make `FrameNumber` 60)) 0.0 "" (struct) "Frame" "Jump"))
  (`MovieSceneSequencePlayer.PlayTo` :`self` _sequenceplayer :`PlaybackParams` (make `MovieSceneSequencePlaybackParams` (make `FrameTime` (make `FrameNumber` 0))))
  (set `self.Have Water` false))

(fn `UserConstructionScript`
  (`parent.UserConstructionScript`))

(fn `WaterHight`
  (params (Fill :type "Float (double-precision)"))
  (`parent.WaterHight` Fill))