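; Thermometer actor (WenDuJi) that plays move-in and move-out animations for "TJT" through a Level Sequence.
; Both functions use one frame range of the LS sequence player: Move In jumps to its start and plays to its end, while Move Out does the reverse.
; BeginPlay and the construction script only call the parent; overlap and Tick events are unused.
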(event `self.ReceiveBeginPlay`
  (`parent.ReceiveBeginPlay`))

(fn `Play Move In TJT`
  (bind _sequenceplayer (`LevelSequenceActor.SequencePlayer` (`self.LS`)))
  (`MovieSceneSequencePlayer.SetPlaybackPosition` _sequenceplayer (make `MovieSceneSequencePlaybackParams` (make `FrameTime` (make `FrameNumber` 160))))
  (`MovieSceneSequencePlayer.PlayTo` :`self` _sequenceplayer :`PlaybackParams` (make `MovieSceneSequencePlaybackParams` (make `FrameTime` (make `FrameNumber` 205)))))

(fn `Play Move Out TJT`
  (bind _sequenceplayer (`LevelSequenceActor.SequencePlayer` (`self.LS`)))
  (`MovieSceneSequencePlayer.SetPlaybackPosition` _sequenceplayer (make `MovieSceneSequencePlaybackParams` (make `FrameTime` (make `FrameNumber` 205))))
  (`MovieSceneSequencePlayer.PlayTo` :`self` _sequenceplayer :`PlaybackParams` (make `MovieSceneSequencePlaybackParams` (make `FrameTime` (make `FrameNumber` 160)))))

(fn `UserConstructionScript`
  (`parent.UserConstructionScript`))