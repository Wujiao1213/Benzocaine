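; BP_TieJiaTai_Zu0 is an iron-stand lab apparatus assembly, apparently a stripped-down variant of its parent.
; On BeginPlay it runs the parent, destroys the pump, round-bottom flask and spherical condenser components, and hides the tube-to-stand component.
; Its construction script passes LSCiLiJiaoBanQi into the magnetic stirrer reached through child component owners.
; An unconnected chain for hiding the condenser and linking its pipe never runs.
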(event `self.ReceiveBeginPlay`
  (`parent.ReceiveBeginPlay`)
  (`ActorComponent.K2_DestroyComponent` (`self.BP_ShuiPeng`))
  (`ActorComponent.K2_DestroyComponent` (`self.BP_YuanDiShaoPing`))
  (`SceneComponent.SetVisibility` (`self.BP_GuanZaoGuanToTieJiaTai`) false false)
  (`ActorComponent.K2_DestroyComponent` (`self.BP_QiuXingLenNing`)))

(fn `UserConstructionScript`
  (`parent.UserConstructionScript`)
  (for _array_element (`SceneComponent.GetChildrenComponents` (`self.BP_CiLiJiaoBanQi`) false)
    (bind _asbp_ci_li_jiao_ban_qi (cast `/Game/BluePrints/BP_CiLiJiaoBanQi` (`ActorComponent.GetOwner` _array_element)))
    (set `/Game/BluePrints/BP_CiLiJiaoBanQi.LS` (`self.LS_CiLiJiaoBanQi`) _asbp_ci_li_jiao_ban_qi)))