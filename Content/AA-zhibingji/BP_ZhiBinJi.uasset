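; Interactive ZhiBinJi machine actor with a hover details panel and a right-click application widget.
; When IsCheak is set, hovering OutLineMesh shows outline and details if OutLineReady, and a right-release at the pressed position opens the application and blocks move input, unless NOAPPLICATION.
; BeginPlay links both widgets to their components; a custom event updates Content and refreshes details.
; The camera look-at timeline is unconnected.
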(event `self.ReceiveBeginPlay`
  (bind _application (`self.Application`))
  (bind _details (`self.Details`))
  (`parent.ReceiveBeginPlay`)
  (`self.SetDetailsToWidget`)
  (bind _aswbp_defult_app (cast `/Game/UI/Actor/WBP_Defult_APP` (`WidgetComponent.GetUserWidgetObject` _application))
    (:`then`
      (set `/Game/UI/Actor/WBP_Defult_APP.parent` _application _aswbp_defult_app))
    (:`CastFailed`
      _))
  (bind _aswbp_details (cast `/Game/UI/WBP_Details` (`WidgetComponent.GetUserWidgetObject` _details))
    (:`then`
      (set `/Game/UI/WBP_Details.parent` _details _aswbp_details))
    (:`CastFailed`
      _))
  (`GameplayStatics.GetActorOfClass` "/Script/LevelSequence.LevelSequenceActor"))

(event `self.OutLineMesh.OnBeginCursorOver`
  (params (TouchedComponent :type "PrimitiveComponent Object Reference"))
  (if (`self.IsCheak`)
    (if (`self.OutLineReady`)
      (`self.OnOutLine`)
      (`SceneComponent.SetVisibility` (`self.Details`) true false))))

(event `self.OutLineMesh.OnEndCursorOver`
  (params (TouchedComponent :type "PrimitiveComponent Object Reference"))
  (`self.OffOutLine`)
  (`SceneComponent.SetVisibility` (`self.Details`) false false))

(event `CustomEvent`)

(event `CustomEvent_1`
  (params (content :type Text))
  ;[1 1 1] 注释
  (set `self.HasContent` true)
  (set `self.Content` content)
  (`self.SetDetailsToWidget`))

(event `self.OutLineMesh.OnClicked`
  (params (TouchedComponent :type "PrimitiveComponent Object Reference") (ButtonPressed :type "Key Structure"))
  ;[1 1 1] 注释
  (bind _returnvalue (`WidgetLayoutLibrary.GetMousePositionOnViewport`))
  (set `self.mousePosition` _returnvalue))

(event `self.OutLineMesh.OnReleased`
  (params (TouchedComponent :type "PrimitiveComponent Object Reference") (ButtonReleased :type "Key Structure"))
  (bind _returnvalue (`GameplayStatics.GetPlayerController` 0))
  (bind _returnvalue_2 (`WidgetLayoutLibrary.GetMousePositionOnViewport`))
  (if (== _returnvalue_2 (`self.mousePosition`))
    (if (not (`SceneComponent.bVisible` (`self.Application`)))
      (if (== ButtonReleased "RightMouseButton")
        (if (`self.IsCheak`)
          (if (not (`self.NOAPPLICATION`))
            (set `self.OutLineReady` false)
            (`SceneComponent.SetVisibility` (`self.Application`) true false)
            (`Controller.SetIgnoreMoveInput` _returnvalue true)
            (`Controller.SetIgnoreLookInput` _returnvalue false)))))))

(event `CustomEvent_2`)

(fn `UserConstructionScript`
  (`parent.UserConstructionScript`))