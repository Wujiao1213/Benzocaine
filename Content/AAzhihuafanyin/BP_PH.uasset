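; BP_PH is a pH-measurement actor with a numeric readout on a widget component.
; When a BP_RuBo actor overlaps OutLineMesh, it plays the LSPH level sequence.
; Two custom events, Time and Time1, each play their own timeline, feeding the animated value into WBP_PH_Num's TextChange every update to animate the displayed number.
; Nothing in this graph calls those two events.
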(event `self.OutLineMesh.OnComponentBeginOverlap`
  (params (OverlappedComponent :type "PrimitiveComponent Object Reference") (OtherActor :type "Actor Object Reference") (OtherComp :type "PrimitiveComponent Object Reference") (OtherBodyIndex :type Integer) (bFromSweep :type Boolean) (SweepResult :type "HitResult Structure (by ref)"))
  (if (== (`GameplayStatics.GetObjectClass` OtherActor) "/Game/BluePrints/BP_RuBo.BP_RuBo_C")
    (`MovieSceneSequencePlayer.Play` (`LevelSequenceActor.SequencePlayer` (`self.LS_PH`)))))

(event `Time`
  (bind _aswbp_ph_num (cast `/Game/UI/Actor/WBP_PH_Num` (`WidgetComponent.GetWidget` (`self.Widget`))))
  (bind (_direction _num) (`Timeline|时间轴_0`)
    (:`Update`
      (`/Game/UI/Actor/WBP_PH_Num.TextChange` _aswbp_ph_num _num))))

(event `Time1`
  (bind _aswbp_ph_num (cast `/Game/UI/Actor/WBP_PH_Num` (`WidgetComponent.GetWidget` (`self.Widget`))))
  (bind (_direction _num1) (`Timeline|时间轴_1`)
    (:`Update`
      (`/Game/UI/Actor/WBP_PH_Num.TextChange` _aswbp_ph_num _num1))))

(fn `UserConstructionScript`
  (`parent.UserConstructionScript`))