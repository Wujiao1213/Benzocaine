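; Quest manager Blueprint that shows the current task prompt and a target marker on screen.
; On BeginPlay it reads the data table row at the current quest index and rebuilds the prompt widget from it.
; TuiJinRenWu increments the index and refreshes the prompt, but nothing in this graph triggers it.
; Releasing R calls RenWuZhuiZong, which recreates the tracking marker widget at a hardcoded zero position.
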(event `self.ReceiveBeginPlay`
  (`self.UpdateDataByIndex`))

(event `Key|R`
  (params (Key :type "Key Structure"))
  (:`Released`
    (`self.RenWuZhuiZong` (0.0 0.0 0.0))))

(fn `RenWuZhuiZong`
  (params (WeiZhi :type "Vector Structure"))
  (bind _w_mubiao (`self.W_MuBiao`)
    (:`then`
      (`Widget.RemoveFromParent` _w_mubiao))
    (:`else`
      _))
  (bind _returnvalue (`|CreateWidget` "/Game/_RenWuXiTon/UI/W_MuBiaoDian.W_MuBiaoDian_C" null WeiZhi))
  (bind _output_get (set `self.W_MuBiao` _returnvalue))
  (`UserWidget.AddToViewport` _output_get 0))

(fn `TuiJinRenWu`
  (`/Engine/EditorBlueprintResources/StandardMacros.IncrementInt` (`self.RenWuSuoYin`)
    (:`  `
      (`self.UpdateDataByIndex`))))

(fn `UpdateDataByIndex`
  (bind _outrownames (`DataTableFunctionLibrary.GetDataTableRowNames` "/Game/_RenWuXiTon/BiaoGe/DataTable_BiaoGe.DataTable_BiaoGe"))
  (bind _returnvalue (`|GetDataTableRow` "/Game/_RenWuXiTon/BiaoGe/DataTable_BiaoGe.DataTable_BiaoGe" (`|GetArrayItem` _outrownames (`self.RenWuSuoYin`)))
    (:`then`
      (bind _w_renwutishi (`self.W_RenWuTiShi`)
        (:`then`
          (`Widget.RemoveFromParent` _w_renwutishi))
        (:`else`
          _))
      (bind _returnvalue_2 (`|CreateWidget` "/Game/_RenWuXiTon/UI/W_RenWuTiShi.W_RenWuTiShi_C" null _returnvalue))
      (bind _output_get (set `self.W_RenWuTiShi` _returnvalue_2))
      (`UserWidget.AddToViewport` _output_get 0))))