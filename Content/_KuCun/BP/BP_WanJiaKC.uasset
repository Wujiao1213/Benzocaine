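; Player inventory (KuCun) that stores BPThing item actors in slots, with keys 1-9 selecting the active slot.
; RuKu fills the first empty slot, parks the actor at a storage location and releases it from the drying oven (GanZaoXiang).
; ChuKu variants move items back into the world by selected slot, class or actor.
; Each change rebuilds the W_KuCun widget from scratch rather than updating it.
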(event `self.ReceiveBeginPlay`
  (`|ExecutionSequence`
    (:`then_1`
      (bind _returnvalue (`|CreateWidget` "/Game/_KuCun/UI/W_KuCun.W_KuCun_C" null self))
      (bind _output_get (set `self.W_KC` _returnvalue))
      (`UserWidget.AddToViewport` _output_get 0))))

(event `Key|One`
  (params (Key :type "Key Structure"))
  (:`Released`
    (set `self.XuanDingIndex` 0)
    (`self.GenXinKuCun`)
    (`self.XianShiMinChen` (`self.XuanDingIndex`) :!label _label)
    (bind _w_ganzaoxiang (`self.W_GanZaoXiang`)
      (:`then`
        (`/Game/UI/Actor/WBP_GanZaoXiang.GenXinAnNiu` _w_ganzaoxiang))
      (:`else`))))

(event `Key|Two`
  (params (Key :type "Key Structure"))
  (:`Released`
    (set `self.XuanDingIndex` 1)
    (`self.GenXinKuCun`)
    (goto _label)))

(event `Key|Three`
  (params (Key :type "Key Structure"))
  (:`Released`
    (set `self.XuanDingIndex` 2)
    (`self.GenXinKuCun`)
    (goto _label)))

(event `Key|Four`
  (params (Key :type "Key Structure"))
  (:`Released`
    (set `self.XuanDingIndex` 3)
    (`self.GenXinKuCun`)
    (goto _label)))

(event `Key|Five`
  (params (Key :type "Key Structure"))
  (:`Released`
    (set `self.XuanDingIndex` 4)
    (`self.GenXinKuCun`)
    (goto _label)))

(event `Key|Six`
  (params (Key :type "Key Structure"))
  (:`Released`
    (set `self.XuanDingIndex` 5)
    (`self.GenXinKuCun`)
    (goto _label)))

(event `Key|Seven`
  (params (Key :type "Key Structure"))
  (:`Released`
    (set `self.XuanDingIndex` 6)
    (`self.GenXinKuCun`)
    (goto _label)))

(event `Key|Eight`
  (params (Key :type "Key Structure"))
  (:`Released`
    (set `self.XuanDingIndex` 7)
    (`self.GenXinKuCun`)
    (goto _label)))

(event `Key|Nine`
  (params (Key :type "Key Structure"))
  (:`Released`
    (set `self.XuanDingIndex` 8)
    (`self.GenXinKuCun`)
    (goto _label)))

(event `SetGanZaoXiang`
  (params (W_GanZaoXiang :type "/Game/UI/Actor/WBP_GanZaoXiang Object Reference"))
  (set `self.W_GanZaoXiang` W_GanZaoXiang))

(fn `ChuKu`
  (params (Location :type "Vector Structure") (Rotation :type "Rotator Structure"))
  (bind (_sweephitresult _returnvalue) (`Actor.K2_SetActorLocationAndRotation` (`.BP_Item_2_FF91E0204E543FC29A3AFAB240C2B131` (break `/Game/_KuCun/Struct/F_ItemSlotX` (`|GetArrayItem` (`self.BP_Thing_SZ`) (`self.XuanDingIndex`)))) Location Rotation false false))
  (if _returnvalue
    (`KismetArrayLibrary.Array_Set` (`self.BP_Thing_SZ`) (`self.XuanDingIndex`) (make `/Game/_KuCun/Struct/F_ItemSlotX` null))
    (`self.GenXinKuCun`)))

(fn `ChuKuByActor`
  (params (Location :type "Vector Structure") (Rotation :type "Rotator Structure") (Actor :type "/Game/BluePrints/BP_Thing Object Reference"))
  (for (_array_element _array_index) (`self.BP_Thing_SZ`)
    (if (== (`.BP_Item_2_FF91E0204E543FC29A3AFAB240C2B131` (break `/Game/_KuCun/Struct/F_ItemSlotX` _array_element)) Actor)
      (bind (_sweephitresult _returnvalue) (`Actor.K2_SetActorLocationAndRotation` Actor Location Rotation false false))
      (if _returnvalue
        (`KismetArrayLibrary.Array_Set` (`self.BP_Thing_SZ`) _array_index (make `/Game/_KuCun/Struct/F_ItemSlotX` null))
        (`self.GenXinKuCun`)
        (break)))))

(fn `ChuKuByClass`
  (params (class :type "Actor Class Reference") (NewLocation :type "Vector Structure") (NewRotation :type "Rotator Structure"))
  (bind (_array_index _found) (`self.FindWuPin` class))
  (if _found
    (bind _bp_item (break `/Game/_KuCun/Struct/F_ItemSlotX` (`|GetArrayItem` (`self.BP_Thing_SZ`) _array_index)))
    (`/Game/_KuCun/UI/W_KuCun.FangZhiXianShi` (`self.W_KC`) _bp_item)
    (bind (_sweephitresult _returnvalue) (`Actor.K2_SetActorLocationAndRotation` _bp_item NewLocation NewRotation false false))
    (if _returnvalue
      (`KismetArrayLibrary.Array_Set` (`self.BP_Thing_SZ`) _array_index (make `/Game/_KuCun/Struct/F_ItemSlotX` null))
      (`self.GenXinKuCun`))))

(fn `FindKongWei`
  (returns (Found :type Boolean) (Index :type Integer))
  (for (_array_element _array_index) (`self.BP_Thing_SZ`)
    (bind (_bp_item _shuliang) (break `/Game/_KuCun/Struct/F_ItemSlotX` _array_element))
    (if (and (not (`KismetSystemLibrary.IsValid` _bp_item)) (== _shuliang 0))
      (return true _array_index)))
  (return false -1))

(fn `FindWuPin`
  (params (class :type "Actor Class Reference"))
  (returns (`Array Index` :type Integer) (Found :type Boolean) (BP_Thing :type "/Game/BluePrints/BP_Thing Object Reference"))
  (for (_array_element _array_index) (`self.BP_Thing_SZ`)
    (bind _bp_item (break `/Game/_KuCun/Struct/F_ItemSlotX` _array_element))
    (if (== (`GameplayStatics.GetObjectClass` _bp_item) class)
      (return _array_index true _bp_item)))
  (return -1 false null))

(fn `FindWuPinByName`
  (params (Name :type Text))
  (returns (`Array Index` :type Integer) (Found :type Boolean) (BP_Thing :type "/Game/BluePrints/BP_Thing Object Reference"))
  (for (_array_element _array_index) (`self.BP_Thing_SZ`)
    (bind _bp_item (break `/Game/_KuCun/Struct/F_ItemSlotX` _array_element))
    (`/Engine/EditorBlueprintResources/StandardMacros.IsValid` _bp_item
      (:`Is Valid`
        (if (`KismetTextLibrary.EqualEqual_TextText` (`/Game/BluePrints/BP_Thing.Name` _bp_item) Name)
          (return _array_index true _bp_item)))))
  (return -1 false null))

(fn `GenXinKuCun`
  (bind _w_kc (`self.W_KC`)
    (:`then`
      (`Widget.RemoveFromParent` _w_kc))
    (:`else`
      _))
  (bind _returnvalue (`|CreateWidget` "/Game/_KuCun/UI/W_KuCun.W_KuCun_C" null self))
  (bind _output_get (set `self.W_KC` _returnvalue))
  (`UserWidget.AddToViewport` _output_get 0))

(fn `RuKu`
  (params (BP_Thing :type "/Game/BluePrints/BP_Thing Object Reference"))
  (bind _bp_thing (`local.BP_Thing`))
  (bind _ganzaoxiangindex (`/Game/BluePrints/BP_Thing.GanZaoXiangIndex` _bp_thing))
  (bind (_found _index) (`self.FindKongWei`))
  (if _found
    (`KismetArrayLibrary.Array_Set` (`self.BP_Thing_SZ`) _index (make `/Game/_KuCun/Struct/F_ItemSlotX` BP_Thing 1))
    (`self.GenXinKuCun`)
    (set `/Game/BluePrints/BP_Thing.JiHuo` false (`local.BP_Thing`))
    (`Actor.K2_SetActorLocation` (`local.BP_Thing`) (`self.KCWZ`) false false)
    (`/Game/_KuCun/UI/W_KuCun.ShiQuXianShi` (`self.W_KC`) (`local.BP_Thing`))
    (if (not (== _ganzaoxiangindex -1))
      (`/Game/BluePrints/BP_GanZaoXiang.NaChu` (`/Game/UI/Actor/WBP_GanZaoXiang.As BP Gan Zao Xiang` (`self.W_GanZaoXiang`)) _ganzaoxiangindex)
      (set `/Game/BluePrints/BP_Thing.GanZaoXiangIndex` -1 _bp_thing))))

(fn `XianShiMinChen`
  (params (Index :type Integer))
  (bind _bp_item (break `/Game/_KuCun/Struct/F_ItemSlotX` (`|GetArrayItem` (`self.BP_Thing_SZ`) Index)))
  (`/Engine/EditorBlueprintResources/StandardMacros.IsValid` _bp_item
    (:`Is Valid`
      (`/Game/_KuCun/UI/W_KuCun.SetName` (`self.W_KC`) _bp_item))))